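; BP_LevelBoundsZone is a box trigger that handles overlaps at level bounds, mostly by sending the overlapping actor to another level.
; In two of the player pawn's driving modes, it starts passenger mode instead.
; Otherwise it sends an open-level-by-name message, choosing a random Destinations entry if the player has a Soul Redirector, else the lonely rock level.
; The random index range includes the array's length, one past the last element.
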(event `self.Box.OnComponentBeginOverlap`
  (params (OverlappedComponent :type "PrimitiveComponent Object Reference") (OtherActor :type "Actor Object Reference") (OtherComp :type "PrimitiveComponent Object Reference") (OtherBodyIndex :type Integer) (bFromSweep :type Boolean) (SweepResult :type "HitResult Structure (by ref)"))
  (bind _destinations (`self.Destinations`))
  (bind _drivingmode (message `/Game/EmPath/Interfaces/BI_GameActions.GetDrivingMode` (`GameplayStatics.GetPlayerPawn` 0)))
  (if (or (`|EnumEquality` _drivingmode "NewEnumerator6") (`|EnumEquality` _drivingmode "NewEnumerator2"))
    (message `/Game/EmPath/Interfaces/BI_GameActions.StartPassengerMode` (`GameplayStatics.GetPlayerPawn` 0))
    (else
      (bind _asmaster (`/Game/HorrorEngine/Blueprints/Core/HorrorEngineFunctions.GetPlayer`))
      (if (`/Game/HorrorEngine/Blueprints/HorrorEngine.HasSoulRedirector` _asmaster)
        (message `/Game/EmPath/Interfaces/BI_GameActions.OpenLevel` OtherActor (`|GetArrayItem` _destinations (`KismetMathLibrary.RandomIntegerInRange` 0 (`KismetArrayLibrary.Array_Length` _destinations))) "0" false false)
        (else
          (message `/Game/EmPath/Interfaces/BI_GameActions.OpenLevel` OtherActor "ul_lonely_rock" "0" false false))))))

(fn `UserConstructionScript`)