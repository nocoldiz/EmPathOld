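; BP_Radio is a usable radio prop that cycles Off, AM, FM and XM bands with a click sound and a preset frequency each.
; While on, Tick evaluates station and static curves at the current frequency, scaled by Volume, to set loudness.
; Both results land on FM1BitcrushStation, so the static curve overrides the station curve when Noise is valid.
; Switching off mutes only the station, and Use just calls its parent.
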(event `self.ReceiveTick`
  (params (DeltaSeconds :type "Float (single-precision)"))
  (bind _frequency (`self.Frequency`))
  (if (not (`|EnumEquality` (`self.RadioType`) "NewEnumerator3"))
    (`|ExecutionSequence`
      (:`then_0`
        (`/Engine/EditorBlueprintResources/StandardMacros.IsValid` (`self.FM1_BitcrushStation`)
          (:`Is Valid`
            (`AudioComponent.SetVolumeMultiplier` (`self.FM1_BitcrushStation`) (* (`CurveFloat.GetFloatValue` (`self.CurveFM1`) _frequency) (`self.Volume`))))))
      (:`then_1`
        (`/Engine/EditorBlueprintResources/StandardMacros.IsValid` (`self.Noise`)
          (:`Is Valid`
            (`AudioComponent.SetVolumeMultiplier` (`self.FM1_BitcrushStation`) (* (`CurveFloat.GetFloatValue` (`self.CurveStatic`) _frequency) (`self.Volume`)))))))))

(event `/Game/EmPath/Interfaces/BI_Radio.CycleFrequency`
  (bind _fm1_bitcrushstation (`self.FM1_BitcrushStation`))
  (`GameplayStatics.PlaySound2D` "/Game/HorrorEngine/Audio/Button/ClickButtonOn_Cue.ClickButtonOn_Cue" 1.0 1.0 0.0 null null)
  (switch `/Game/EmPath/Enum/E_Radio` (`self.RadioType`)
    (:`NewEnumerator3`
      (set `self.RadioType` "NewEnumerator0")
      (set `self.Frequency` 420.0)
      (`AudioComponent.SetVolumeMultiplier` _fm1_bitcrushstation 0.4)
      (`AudioComponent.SetVolumeMultiplier` (`self.Noise`) 0.4))
    (:`NewEnumerator0`
      (set `self.RadioType` "NewEnumerator1")
      (set `self.Frequency` 32.0))
    (:`NewEnumerator1`
      (set `self.RadioType` "NewEnumerator2")
      (set `self.Frequency` 1.0))
    (:`NewEnumerator2`
      (set `self.RadioType` "NewEnumerator3")
      (`AudioComponent.SetVolumeMultiplier` _fm1_bitcrushstation 0.0))))

(event `/Game/EmPath/Interfaces/BI_Radio.SetFrequency`
  (params (Frequency :type "Float (double-precision)"))
  (set `self.Frequency` Frequency))

(fn `Use`
  (params (HorrorEvent :type Boolean))
  (`parent.Use` HorrorEvent))

(fn `UserConstructionScript`
  (`parent.UserConstructionScript`))