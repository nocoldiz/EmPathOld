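; Spell compressor object that holds one registered spell, apparently as part of a spell ritual.
; RegisterSpell stores the spell, async-loads its travel particle and shows it on the Niagara components.
; FinishRitual clears the Niagara asset but leaves the stored spell intact.
; GetStoredSpell returns that spell with an IsDominant flag, while RecordNewSpell is an empty event.
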(event `/Game/EmPath/Interfaces/BI_SpellCompressor.RecordNewSpell`)

(event `/Game/EmPath/Interfaces/BI_SpellCompressor.RegisterSpell`
  (params (Spell :type "/Game/EmPath/Structures/Spell/S_Spell Structure"))
  (bind (_data _physics _castoptions _travel) (break `/Game/EmPath/Structures/Spell/S_Spell` Spell))
  (set `self.StoredSpell` Spell)
  (`|LoadAsset` (`.Particle_33_CB2C16674D837A32B01A6EB05D403AC0` (break `/Game/EmPath/Structures/Spell/S_SpellPhase` _travel))
    (:`Completed`
      (`NiagaraComponent.SetAsset` (`self.Niagara`) (`|ConvertAsset` (`.Particle_33_CB2C16674D837A32B01A6EB05D403AC0` (break `/Game/EmPath/Structures/Spell/S_SpellPhase` _travel))) true)
      (`NiagaraComponent.SetAsset` (`self.Niagara`) (`|ConvertAsset` (`.Particle_33_CB2C16674D837A32B01A6EB05D403AC0` (break `/Game/EmPath/Structures/Spell/S_SpellPhase` _travel))) true))))

(event `/Game/EmPath/Interfaces/BI_SpellCompressor.FinishRitual`
  (`NiagaraComponent.SetAsset` (`self.Niagara`) null true))

(fn `GetStoredSpell`
  (returns (SpellInfo :type "/Game/EmPath/Structures/Spell/S_Spell Structure") (IsDominant :type Boolean))
  (return (`self.StoredSpell`) (`self.IsDominant`)))

(fn `UserConstructionScript`
  (`parent.UserConstructionScript`))