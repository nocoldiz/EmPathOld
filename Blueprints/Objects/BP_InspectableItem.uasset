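; Inspectable world item, optionally buyable, that the player can pay for through its inspection action.
; Construction runs the parent and HM default setup, then applies mesh, inspection and inventory settings.
; When Buyable, InspectionUse reads the pawn's money, deducts Price if affordable and plays a cash sound, without granting the item.
; Use only prints a debug string; the other interaction events and the construction-time Buyable branch are empty.
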(event `/Game/HorrorEngine/Blueprints/Core/Use.AlternativeUse`
  (params (HorrorEvent :type Boolean))
  ;[1 1 1] Buy item
)

(event `self.InspectionUse`
  (bind _returnvalue (`GameplayStatics.GetPlayerPawn` 0))
  (bind _price (`self.Price`))
  ;[1 1 1] Buy item
  (if (`self.Buyable`)
    (bind _money (message `/Game/EmPath/Interfaces/BI_GameActions.GetMoney` _returnvalue))
    (if (>= _money _price)
      (message `/Game/EmPath/Interfaces/BI_GameActions.SetMoney` _returnvalue (- _money _price))
      (`/Game/HorrorEngine/Blueprints/Core/HorrorEngineMacros.HM_2DSound` "/Game/EmPath/Sounds/Cash.Cash" true))))

(event `/Game/HorrorEngine/Blueprints/Core/Use.Use`
  (params (HorrorEvent :type Boolean))
  (`KismetSystemLibrary.PrintString` "Hello"))

(event `self.InventoryUse`)

(event `self.AddToCache`)

(event `self.Retake`
  (params (InventorySave :type "/Game/HorrorEngine/Blueprints/Structures/SaveStructures/InventorySave Structure")))

(fn `UserConstructionScript`
  (`parent.UserConstructionScript`)
  (`/Game/HorrorEngine/Blueprints/Core/HorrorEngineMacros.HM_DefaultConstructions` (`self.CreateNewHorrorEvent`))
  (`/Game/HorrorEngine/Blueprints/Core/HorrorEngineFunctions.SetMesh` (`self.Actor`) (`self.MeshSettings`))
  (`self.SetInspection` (`self.InspectionSettings`))
  (`self.SetInventory` (`self.InventorySettings`))
  (if (`self.Buyable`)
    _))