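; BP_KillingGround is a hazard area that burns and destroys damageable or object actors standing inside it when activated.
; ActivateKillingGround checks everything overlapping its CollisionBox for the BPI_Damagable or BI_Object interface.
; Each match gets a fire Niagara effect and sound at its location, then is destroyed, with a random Delay looping back into the destroy call.
; GetStoredSpell is a stub that reports non-dominant.
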(event `self.ReceiveActorBeginOverlap`
  (params (OtherActor :type "Actor Object Reference"))
  (`KismetArrayLibrary.Array_AddUnique` (`self.Other Actor`) OtherActor))

(event `/Game/EmPath/Interfaces/BI_SpellCompressor.ActivateKillingGround`
  (`KismetSystemLibrary.PrintString` "Kill")
  (for _array_element (`PrimitiveComponent.GetOverlappingActors` (`self.CollisionBox`) null)
    (if (`KismetSystemLibrary.DoesImplementInterface` _array_element "/Game/EmPath/Interfaces/BPI_Damagable.BPI_Damagable_C")
      (bind _returnvalue (`self.K2_GetActorLocation` _array_element))
      (`NiagaraFunctionLibrary.SpawnSystemAtLocation` "/Game/M5VFXVOL2/Niagara/Reference/Fire/4_Nbigfire_fwd_vg_pt.4_Nbigfire_fwd_vg_pt" _returnvalue :!label _label)
      (`GameplayStatics.SpawnSoundAtLocation` "/Game/StarterContent/Audio/Fire01.Fire01" _returnvalue (struct) 1.0 1.0 0.0 null null)
      (`self.K2_DestroyActor` _array_element :!label _label_2)
      (`KismetSystemLibrary.Delay` (`KismetMathLibrary.RandomFloatInRange` 3.0 8.0))
      (goto _label_2)
      (elif (`KismetSystemLibrary.DoesImplementInterface` _array_element "/Game/EmPath/Interfaces/BI_Object.BI_Object_C")
        (goto _label)))))

(fn `GetStoredSpell`
  (returns (SpellInfo :type "/Game/EmPath/Structures/Spell/S_Spell Structure") (IsDominant :type Boolean))
  (return (struct) false))

(fn `UserConstructionScript`)