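; Spell vending machine that displays spellbooks on sockets and lets them drop when one is requested.
; BeginPlay spawns machine-owned books at the sockets, with gravity and physics simulation off, using CreateRandomSpell, which is currently empty.
; GetSpellbookVendingMachine decrements the stored count and re-enables gravity on every spellbook it owns, not just one.
; Ritual events and the other spell functions are unimplemented stubs.
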(event `/Game/EmPath/Interfaces/BI_Spellcrafting.GetSpellbookVendingMachine`
  (params (Index :type Integer))
  (`/Engine/EditorBlueprintResources/StandardMacros.DecrementInt` (`self.StoredBooks`)
    (:`  `
      (bind _outactors (`GameplayStatics.GetAllActorsOfClass` "/Game/EmPath/Blueprints/Objects/BP_Spellbook.BP_Spellbook_C"))
      (for _array_element _outactors
        (if (== (`self.GetOwner` _array_element) self)
          (bind _asbp_spellbook (cast `/Game/EmPath/Blueprints/Objects/BP_Spellbook` _array_element))
          (`PrimitiveComponent.SetEnableGravity` (`/Game/HorrorEngine/Blueprints/Core/PhysicsObject.PhysicsObject` _asbp_spellbook) true))))))

(event `Placebook`
  (params (Index :type Integer) (SpellInfo :type "/Game/EmPath/Structures/Spell/S_Spell Structure"))
  (bind _returnvalue (`|SpawnActorFromClass` "/Game/EmPath/Blueprints/Objects/BP_Spellbook.BP_Spellbook_C" (`SceneComponent.GetSocketTransform` (`self.Actor`) (`|GetArrayItem` (`self.Sockets`) Index) "RTS_World") "AlwaysSpawn" "MultiplyWithRoot" self SpellInfo "NewEnumerator167" false false "Spellbook" null))
  (bind _asbp_spellbook (cast `/Game/EmPath/Blueprints/Objects/BP_Spellbook` _returnvalue))
  (`PrimitiveComponent.SetEnableGravity` (`/Game/HorrorEngine/Blueprints/Core/PhysicsObject.PhysicsObject` _asbp_spellbook) false))

(event `self.ReceiveBeginPlay`
  (for _index (range (+ (`self.MaxBooks`) 1))
    (bind _spell (`/Game/EmPath/Interfaces/BI_Spellcrafting.CreateRandomSpell` 0))
    (`self.Placebook` _index _spell)))

(event `/Game/EmPath/Interfaces/BI_Spellcrafting.InitiateRitual`)

(event `/Game/EmPath/Interfaces/BI_Spellcrafting.RecordNewSpell`)

(event `/Game/EmPath/Interfaces/BI_Spellcrafting.FinishRitual`)

(event `CreateSpell_1_1`
  (params (SpellName :type "/Game/EmPath/Enum/E_SpellNames Enum" :default "NewEnumerator0")))

(fn `CompressSpell`
  (params (DominantSpell :type "/Game/EmPath/Enum/E_SpellNames Enum" :default "NewEnumerator0") (SecondarySpell :type "/Game/EmPath/Enum/E_SpellNames Enum" :default "NewEnumerator0"))
  (returns (Spell :type "/Game/EmPath/Structures/Spell/S_Spell Structure"))
  (return))

(fn `CreateRandomSpell`
  (params (ChaosFactor :type Integer))
  (returns (Spell :type "/Game/EmPath/Structures/Spell/S_Spell Structure")))

(fn `CreateSpell`
  (params (SpellName :type "/Game/EmPath/Enum/E_SpellNames Enum" :default "NewEnumerator0"))
  (returns (Spell :type "/Game/EmPath/Structures/Spell/S_Spell Structure"))
  (return))

(fn `GetStoredSpell`
  (returns (SpellInfo :type "/Game/EmPath/Structures/Spell/S_Spell Structure") (IsDominant :type Boolean))
  (return (struct) false))

(fn `UserConstructionScript`
  (`parent.UserConstructionScript`))