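; BP_Object is the general-purpose physics item the player can hold, rotate, zoom, inspect, unpack, use and store in the backpack.
; The construction script sets mesh, physics and weapon hold offsets; Use switches on ObjectType for liquid, distance-based melee, steering wheel, pillow or broom actions.
; Hold and release extend parent logic, while TakeItem adds the item's DT_Backpack row and hides the actor.
; ApplyEffect clones or glassifies it; health and combat functions are stubs.
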(event `LiquidContainer`
  (`GameplayStatics.PlaySound2D` null 1.0 1.0 0.0 null null)
  (switch `/Game/EmPath/Enum/E_LiquidTypes` (`self.LiquidType`)))

(event `Inspect`
  (bind _returnvalue (`GameplayStatics.GetPlayerPawn` 0))
  (bind _dialogwidget (`self.DialogWidget`))
  ;[1 1 1] Inspect item
  (if (`self.ShouldRemove`)
    ;[1 1 1] Remove Widgey
    (`/Engine/EditorBlueprintResources/StandardMacros.IsValid` _dialogwidget
      (:`Is Valid`
        (`/Game/EmPath/UI/WB_DialogBox.RemoveWidgetNoDelay` _dialogwidget)
        (set `self.ShouldRemove` false)))
    (else
      (bind _dialogstate (message `/Game/EmPath/Interfaces/BI_GameActions.GetIsTalking` _returnvalue))
      (if (`|EnumEquality` _dialogstate "NewEnumerator1")
        ;[1 1 1] Speed up dialogue
        (`/Engine/EditorBlueprintResources/StandardMacros.IsValid` _dialogwidget
          (:`Is Valid`
            (set `self.ShouldRemove` true)))
        (else
          (message `/Game/EmPath/Interfaces/BI_GameActions.StartTalking` _returnvalue "NewEnumerator0")
          ;[1 1 1] Create widget
          (bind _returnvalue_2 (`|CreateWidget` "/Game/EmPath/UI/WB_DialogBox.WB_DialogBox_C" null "" true 0.0 (`self.Price`)))
          (`UserWidget.AddToViewport` _returnvalue_2 0))))))

(event `self.Use`
  (params (HorrorEvent :type Boolean))
  (bind _objecttype (`self.ObjectType`))
  (if (not (`self.DisableUseFromWorld`))
    (`KismetSystemLibrary.PrintString` (`|GetEnumeratorNameAsString` _objecttype) :!label _label)
    ;[1 1 1] Unpacking
    (if (`self.Packed`)
      (set `self.Packed` false)
      (`GameplayStatics.PlaySound2D` (`self.UnpackSound`) 0.5 1.0 0.0 null null)
      (`SceneComponent.K2_SetWorldRotation` (`self.PhysicsObject`) (`KismetMathLibrary.FindLookAtRotation` (`self.GetActorForwardVector` (`GameplayStatics.GetPlayerCameraManager` 0)) (`self.K2_GetActorLocation`)) false false)
      (`/Game/HorrorEngine/Blueprints/Core/HorrorEngineFunctions.SetMesh` (`self.PhysicsObject`) (`self.MeshSettings`))
      (else
        ;[1 1 1] Object Actions
        (switch `/Game/EmPath/Enum/E_ObjectTypes` _objecttype
          (:`NewEnumerator1`
            (`self.LiquidContainer`))
          (:`NewEnumerator32`
            (if (not (`self.DisableAttack`))
              (`self.Melee`)))
          (:`NewEnumerator33`
            (`self.SteeringWheel`))
          (:`NewEnumerator34`
            (`self.Pillow`))
          (:`NewEnumerator35`
            (`self.Broom`)))))))

(event `Key|MouseScrollUp`
  (params (Key :type "Key Structure"))
  (bind _heldslot (`self.HeldSlot`))
  (bind (_heldlocation_x _heldlocation_y _heldlocation_z) (`KismetMathLibrary.BreakVector` (`self.HeldLocation`)))
  (bind _relativelocation_x (`KismetMathLibrary.BreakVector` (`SceneComponent.RelativeLocation` _heldslot)))
  (bind _returnvalue (`KismetMathLibrary.FClamp` (+ _relativelocation_x (`self.ZoomSpeed`)) (`self.MinZoom`) (`self.MaxZoom`)))
  ;[1 1 1] Zoom Settings
  (:`Pressed`
    (`/Game/HorrorEngine/Blueprints/Core/HorrorEngineMacros.HM_CheckInteraction`)
    (bind _output_get (set `self.ObjectDistance` _returnvalue))
    (`SceneComponent.K2_SetRelativeLocation` _heldslot (`KismetMathLibrary.MakeVector` _returnvalue _heldlocation_y _heldlocation_z) false false)
    ;[1 1 1] Use Settings
    (`KismetSystemLibrary.PrintString` (`KismetStringLibrary.Conv_DoubleToString` _output_get))))

(event `InputAction|[HE]Use`
  (params (Key :type "Key Structure"))
  (:`Pressed`
    ;[1 1 1] Object Actions
    (set `self.IsUsing` true)
    (goto _label))
  (:`Released`
    (set `self.IsUsing` false)
    (bind _asmaster (`/Game/HorrorEngine/Blueprints/Core/HorrorEngineFunctions.GetPlayer`))
    (if (`|EnumEquality` (`self.ObjectType`) "NewEnumerator32")
      (set `/Game/HorrorEngine/Blueprints/HorrorEngine.RotateHeldItem` false _asmaster)
      (else
        (set `/Game/HorrorEngine/Blueprints/HorrorEngine.RotateHeldItem` false _asmaster)))))

(event `self.Shoot`
  (params (HorrorEvent :type Boolean))
  ;[1 1 1] Use Settings
  (`self.ShootObject`))

(event `Key|MouseScrollDown`
  (params (Key :type "Key Structure"))
  (bind (_heldlocation_x _heldlocation_y _heldlocation_z) (`KismetMathLibrary.BreakVector` (`self.HeldLocation`)))
  (bind _heldslot (`self.HeldSlot`))
  (bind _relativelocation_x (`KismetMathLibrary.BreakVector` (`SceneComponent.RelativeLocation` _heldslot)))
  (bind _returnvalue (`KismetMathLibrary.FClamp` (- _relativelocation_x (`self.ZoomSpeed`)) (`self.MinZoom`) (`self.MaxZoom`)))
  ;[1 1 1] Zoom Settings
  (:`Pressed`
    (`/Game/HorrorEngine/Blueprints/Core/HorrorEngineMacros.HM_CheckInteraction`)
    (set `self.ObjectDistance` _returnvalue)
    (`SceneComponent.K2_SetRelativeLocation` _heldslot (`KismetMathLibrary.MakeVector` _returnvalue _heldlocation_y _heldlocation_z) false false)))

(event `Melee`
  (bind _physicsobject (`self.PhysicsObject`))
  (bind (_relativelocation_x _relativelocation_y _relativelocation_z) (`KismetMathLibrary.BreakVector` (`SceneComponent.RelativeLocation` (`self.PhysicsObject`))))
  (bind (_returnvalue_x _returnvalue_y _returnvalue_z) (`KismetMathLibrary.BreakVector` (+ (* (`self.GetActorForwardVector` (`GameplayStatics.GetPlayerCameraManager` 0)) 200.0) (`SceneComponent.RelativeLocation` _physicsobject))))
  ;[1 1 1] Melee attack
  (bind _asmaster (`/Game/HorrorEngine/Blueprints/Core/HorrorEngineFunctions.GetPlayer`))
  (if (<= (`self.ObjectDistance`) 120.0)
    (`KismetSystemLibrary.MoveComponentTo` (`self.PhysicsObject`) (`KismetMathLibrary.MakeVector` _returnvalue_x _returnvalue_y _returnvalue_z) (`SceneComponent.RelativeRotation` _physicsobject) true true 0.08)
    (`KismetSystemLibrary.Delay` 0.08)
    (set `self.DisableAttack` false)
    (elif (<= (`self.ObjectDistance`) 200.0)
      (set `/Game/HorrorEngine/Blueprints/HorrorEngine.RotateHeldItem` true _asmaster) ; Rotate
      (else
        (set `self.DisableAttack` true)
        (`GameplayStatics.PlaySoundAtLocation` "/Game/EmPath/Sounds/axe-swing.axe-swing" (`SceneComponent.RelativeLocation` (`self.PhysicsObject`)) (struct) 1.0 1.0 0.0 null null null null)
        ;;[1 1 1] LongRange
        (`KismetSystemLibrary.MoveComponentTo` (`self.PhysicsObject`) (`KismetMathLibrary.MakeVector` _relativelocation_x _relativelocation_y _relativelocation_z) (* (`KismetMathLibrary.RandomRotator` true) 12.0))
        (`KismetSystemLibrary.Delay` 0.1)
        (set `self.DisableAttack` false)))))

(event `Key|LeftShift`
  (params (Key :type "Key Structure"))
  ;[1 1 1] Fix Object
  (:`Pressed`
    (if (not (`self.SoundCooldown`))
      (`/Game/HorrorEngine/Blueprints/Core/HorrorEngineMacros.HM_CheckInteraction`)
      (`PrimitiveComponent.SetSimulatePhysics` (`self.PhysicsObject`) false)
      (set `self.SoundCooldown` true)
      (`self.ReleaseObject`))))

(event `self.RotateItem`
  (params (A :type "Float (double-precision)") (A2 :type "Float (double-precision)"))
  (if (`|EnumEquality` (`self.ObjectType`) "NewEnumerator32")
    ;[1 1 1] Normal rotation
    (`SceneComponent.K2_SetRelativeRotation` (`self.HeldSlot`) (`KismetMathLibrary.ComposeRotators` (`SceneComponent.RelativeRotation` (`self.HeldSlot`)) (* (`KismetMathLibrary.MakeRotator` 0.0 (* A 1.0) (* A2 -1.0)) (`self.RotationSpeed`))) false false)
    (else
      ;[1 1 1] Normal rotation
      (`SceneComponent.K2_SetRelativeRotation` (`self.HeldSlot`) (`KismetMathLibrary.ComposeRotators` (`SceneComponent.RelativeRotation` (`self.HeldSlot`)) (* (`KismetMathLibrary.MakeRotator` 0.0 (* A 1.0) (* A2 -1.0)) (`self.RotationSpeed`))) false false))))

(event `InputAction|[HE]Reload`
  (params (Key :type "Key Structure"))
  (bind _heldslot (`self.HeldSlot`))
  (bind (_x _y _z) (`KismetMathLibrary.BreakRotIntoAxes` (`SceneComponent.RelativeRotation` _heldslot)))
  ;[1 1 1] Rotate Object
  (:`Pressed`
    (`SceneComponent.K2_SetRelativeRotation` _heldslot (`KismetMathLibrary.MakeRotationFromAxes` _x _y (- _z (0.0 0.0 -90.0))) false false)))

(event `Pillow`
  (message `/Game/EmPath/Interfaces/BI_GameActions.GoToSleep` (`GameplayStatics.GetPlayerPawn` 0)))

(event `InputAction|[HE]RotateObject`
  (params (Key :type "Key Structure"))
  ;[1 1 1] Enable rotation
  (:`Pressed`
    (bind _asmaster (`/Game/HorrorEngine/Blueprints/Core/HorrorEngineFunctions.GetPlayer`))
    (set `/Game/HorrorEngine/Blueprints/HorrorEngine.RotateHeldItem` true _asmaster))
  (:`Released`
    (bind _asmaster_2 (`/Game/HorrorEngine/Blueprints/Core/HorrorEngineFunctions.GetPlayer`))
    (set `/Game/HorrorEngine/Blueprints/HorrorEngine.RotateHeldItem` false _asmaster_2)))

(event `Broom`
  (bind _returnvalue (`GameplayStatics.GetPlayerPawn` 0))
  ;[1 1 1] Broom
  (`/Engine/EditorBlueprintResources/StandardMacros.FlipFlop`
    (:`A`
      (message `/Game/EmPath/Interfaces/BI_GameActions.SetDrivingMode` _returnvalue "NewEnumerator8"))
    (:`B`
      (message `/Game/EmPath/Interfaces/BI_GameActions.SetDrivingMode` _returnvalue "NewEnumerator1"))))

(event `SteeringWheel`
  (bind _returnvalue (`GameplayStatics.GetPlayerPawn` 0))
  ;[1 1 1] SteeringWHeel
  (message `/Game/EmPath/Interfaces/BI_GameActions.StopSeating` _returnvalue (0.0 0.0 0.0) _returnvalue))

(event `Diary`)

(event `Retake`
  (params (InventorySave :type "/Blueprints/Objects/BP_Object Object Reference"))
  (`KismetSystemLibrary.PrintString` "Retake")
  (`self.TakeItem`))

(event `self.ReleaseObject`
  ;[1 1 1] Release Object
  (`|ExecutionSequence`
    (:`then_0`
      (switch `/Game/EmPath/Enum/E_ObjectTypes` (`self.ObjectType`)
        (:`NewEnumerator35`
          (`self.DropBroom`))))
    (:`then_1`
      (`parent.ReleaseObject`)
      (`NiagaraComponent.SetAsset` (`self.Particle`) null true))))

(event `self.HeldObject`
  (params (HitResult :type "HitResult Structure"))
  ;[1 1 1] Held Object
  (`|ExecutionSequence`
    (:`then_0`
      (switch `/Game/EmPath/Enum/E_ObjectTypes` (`self.ObjectType`)))
    (:`then_1`
      (`parent.HeldObject` (struct))
      (`NiagaraComponent.SetAsset` (`self.Particle`) null true))))

(event `/Game/EmPath/Interfaces/BI_Object.Apply Effect`
  (params (Status :type "/Game/EmPath/Enum/E_SpellEffect Enum" :default "NewEnumerator12") (Duration :type "Float (double-precision)") (Magnitude :type "Float (double-precision)") (Enable :type Boolean) (SuccessRate :type "Float (double-precision)"))
  (switch `/Game/EmPath/Enum/E_SpellEffect` Status
    (:`NewEnumerator39`
      (`|SpawnActorFromClass` "BP_Object_C" (`self.GetTransform`) "AdjustIfPossibleButAlwaysSpawn" "MultiplyWithRoot" null false null "/Game/EmPath/Sounds/SC_Unpack.SC_Unpack" true false "Object" null))
    (:`NewEnumerator24`
      (`PrimitiveComponent.SetMaterial` (`self.PhysicsObject`) 0 "/DatasmithContent/Materials/FBXImporter/VRED/Glass.Glass"))))

(fn `AlternativeUse`
  (params (HorrorEvent :type Boolean))
  (`parent.AlternativeUse` HorrorEvent))

(fn `DropBroom`
  (bind _returnvalue (`GameplayStatics.GetPlayerPawn` 0))
  (bind _drivingmode (message `/Game/EmPath/Interfaces/BI_GameActions.GetDrivingMode` _returnvalue))
  (if (`|EnumEquality` _drivingmode "NewEnumerator8")
    (message `/Game/EmPath/Interfaces/BI_GameActions.SetDrivingMode` _returnvalue "NewEnumerator1")))

(fn `GetCurrentHealth`
  (returns (Health :type "Float (double-precision)"))
  (return 0.0))

(fn `GetInfo`
  (returns (Name :type Text))
  (return (`self.Name`)))

(fn `GetMaxHealth`
  (returns (MaxHealth :type "Float (double-precision)"))
  (return 0.0))

(fn `GetTeamNumber`
  (returns (TeamNumber :type Integer))
  (return 0))

(fn `Heal`
  (params (Amount :type "Float (double-precision)" :default 0.0))
  (returns (NewHealth :type "Float (double-precision)"))
  (return 0.0))

(fn `IsAttacking`
  (returns (Attacking :type Boolean))
  (return false))

(fn `IsDead`
  (returns (Dead :type Boolean))
  (return false))

(fn `ReserveAttackToken`
  (params (Amount :type Integer :default 0))
  (returns (Success :type Boolean))
  (return false))

(fn `TakeDamage`
  (params (DamageInfo :type "/Game/EmPath/Structures/S_DamageInfo Structure") (`Damage Causer` :type "Actor Object Reference"))
  (returns (WasDamaged :type Boolean))
  (return false))

(fn `TakeItem`
  (locals (ValidItems :type Integer :default 8) (FirstUnvalid :type Integer))
  (bind _name (`self.Name`))
  (set `local.ValidItems` 0)
  (bind _asmaster (`/Game/HorrorEngine/Blueprints/Core/HorrorEngineFunctions.GetPlayer`))
  (bind _playerbackpack (`/Game/HorrorEngine/Blueprints/HorrorEngine.PlayerBackpack` _asmaster))
  ;[1 1 1] Count valid items
  (for (_ _array_index) _playerbackpack
    (`/Engine/EditorBlueprintResources/StandardMacros.IsValid` null
      (:`Is Valid`
        (`/Engine/EditorBlueprintResources/StandardMacros.IncrementInt` (`local.ValidItems`)))
      (:`Is Not Valid`
        (`/Engine/EditorBlueprintResources/StandardMacros.DoOnce` false
          (:`Completed`
            (set `local.FirstUnvalid` _array_index))))))
  (if (>= (`local.ValidItems`) 8)
    (`/Game/HorrorEngine/Blueprints/Core/HorrorEngineFunctions.Notice` "Backpack is full")
    (else
      (`/Engine/EditorBlueprintResources/StandardMacros.IsValid` null
        (:`Is Valid`
          _)
        (:`Is Not Valid`
          _))
      (`/Game/HorrorEngine/Blueprints/Core/HorrorEngineFunctions.Notice` "" _name "added to backpack")
      (bind _returnvalue (`|GetDataTableRow` "/Game/EmPath/DataTables/DT_Backpack.DT_Backpack" (`KismetStringLibrary.Conv_StringToName` (`KismetTextLibrary.Conv_TextToString` _name)))
        (:`then`
          (`KismetArrayLibrary.Array_Add` _playerbackpack _returnvalue)
          (`self.SetActorHiddenInGame` true)
          (`parent.TakeItem`)
          (`SceneComponent.K2_SetWorldLocation` (`self.PhysicsObject`) (0.0 0.0 -9999.0) false true))))))

(fn `UserConstructionScript`
  (bind _packedmesh (`self.PackedMesh`))
  (bind (_meshsettings_mesh _meshsettings_materialsettings) (break `/Game/HorrorEngine/Blueprints/Structures/SetMesh/SetMesh` (`self.MeshSettings`)))
  (`parent.UserConstructionScript`)
  (`/Game/HorrorEngine/Blueprints/Core/HorrorEngineMacros.HM_DefaultConstructions` (`self.CreateNewHorrorEvent`))
  (if (not (> (`KismetArrayLibrary.Array_Length` (`self.AlternateMeshes`)) 0))
    (if (`self.Packed`)
      (`KismetSystemLibrary.LoadAsset_Blocking` _packedmesh)
      (`/Game/HorrorEngine/Blueprints/Core/HorrorEngineFunctions.SetMesh` (`self.PhysicsObject`) (make `/Game/HorrorEngine/Blueprints/Structures/SetMesh/SetMesh` (`|ConvertAsset` _packedmesh) _meshsettings_materialsettings))
      (else
        (`/Game/HorrorEngine/Blueprints/Core/HorrorEngineFunctions.SetMesh` (`self.PhysicsObject`) (`self.MeshSettings`))))
    (`self.SetPhysicsSettings` (`self.PhysicsSettings`))
    (switch `/Game/EmPath/Enum/E_ObjectTypes` (`self.ObjectType`)
      (:`NewEnumerator31`
        _)
      (:`NewEnumerator32`
        _))
    (set `self.HeldLocation` (100.0 60.0 10.0))
    (set `self.CenterOfMass` (0.0 -10.0 -100.0))))