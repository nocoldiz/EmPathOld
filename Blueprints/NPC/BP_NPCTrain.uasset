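; BP_NPCTrain is an NPC, apparently a train passenger, with a randomized look, voice pitch and travel dialogue.
; Construction picks a random flipbook and pitch, then fills DialogLines and Topics from randomly drawn DT_TravelDialogue rows, which may repeat.
; On BeginPlay it destroys itself when a random roll falls below Rarity, so higher values mean fewer appearances.
; Topic widget setup and range-based visibility logic are disconnected and never run.
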(event `self.ReceiveBeginPlay`
  (if (< (`KismetMathLibrary.RandomFloatInRange` 0.0 1.0) (`self.Rarity`))
    (`self.K2_DestroyActor`)))

(event `self.TopicRange.OnComponentBeginOverlap`
  (params (OverlappedComponent :type "PrimitiveComponent Object Reference") (OtherActor :type "Actor Object Reference") (OtherComp :type "PrimitiveComponent Object Reference") (OtherBodyIndex :type Integer) (bFromSweep :type Boolean) (SweepResult :type "HitResult Structure (by ref)")))

(event `self.TopicRange.OnComponentEndOverlap`
  (params (OverlappedComponent :type "PrimitiveComponent Object Reference") (OtherActor :type "Actor Object Reference") (OtherComp :type "PrimitiveComponent Object Reference") (OtherBodyIndex :type Integer)))

(fn `UserConstructionScript`
  (`parent.UserConstructionScript`)
  (`PaperFlipbookComponent.SetFlipbook` (`self.Sprite`) (`KismetArrayLibrary.Array_Random` (`self.Sprites`)))
  (set `self.Pitch` (`KismetMathLibrary.RandomFloatInRange` 0.4 1.4))
  (bind _outrownames (`DataTableFunctionLibrary.GetDataTableRowNames` "/Game/EmPath/DataTables/DT_TravelDialogue.DT_TravelDialogue"))
  (for _ (range 6)
    (bind _returnvalue (`|GetDataTableRow` "/Game/EmPath/DataTables/DT_TravelDialogue.DT_TravelDialogue" (`KismetArrayLibrary.Array_Random` _outrownames))
      (:`then`
        (bind (_dialogue _topic) (break `/Game/EmPath/Structures/ST_Dialogue` _returnvalue))
        (`KismetArrayLibrary.Array_Add` (`self.DialogLines`) _dialogue)
        (`KismetArrayLibrary.Array_Add` (`self.Topics`) _topic)))))