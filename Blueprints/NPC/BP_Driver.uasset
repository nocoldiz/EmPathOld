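; BP_Driver is an interactable NPC, "Bubba", who opens a dialogue box when the player uses it.
; Construction runs the HM horror-event defaults and sets meshes for the Interact and Button components.
; Use runs the HM interaction check, then Talk, which checks the pawn's talking state to either speed up the current dialogue or start talking and create a WB_DialogBox with its own voice pitch.
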(event `self.Use`
  (params (HorrorEvent :type Boolean))
  ;[1 1 1] Interact Settings
  (`/Game/HorrorEngine/Blueprints/Core/HorrorEngineMacros.HM_CheckInteraction`)
  (`self.Talk`))

(fn `Talk`
  (bind _returnvalue (`GameplayStatics.GetPlayerPawn` 0))
  (bind _dialogstate (message `/Game/EmPath/Interfaces/BI_GameActions.GetIsTalking` _returnvalue))
  (if (`|EnumEquality` _dialogstate "NewEnumerator1")
    (`/Game/EmPath/UI/WB_DialogBox.SpeedUpDialogue` (`self.Widget`))
    (else
      (message `/Game/EmPath/Interfaces/BI_GameActions.StartTalking` _returnvalue "NewEnumerator1")
      (bind _returnvalue_2 (`|CreateWidget` :`Class` "/Game/EmPath/UI/WB_DialogBox.WB_DialogBox_C" :`Pitch` 0.7 :`NpcName` "Bubba" :`NPC` null :`NewVar` null))
      (set `self.Widget` _returnvalue_2)
      (`UserWidget.AddToViewport` _returnvalue_2 0))))

(fn `UserConstructionScript`
  (`/Game/HorrorEngine/Blueprints/Core/HorrorEngineMacros.HM_DefaultConstructions` (`self.CreateNewHorrorEvent`))
  (`/Game/HorrorEngine/Blueprints/Core/HorrorEngineFunctions.SetMesh` (`self.Interact`) (`self.ButtonBaseMesh`))
  (`/Game/HorrorEngine/Blueprints/Core/HorrorEngineFunctions.SetMesh` (`self.Button`)))