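; Interactive radio prop for a horror game that toggles on and off with Use and cycles channels, with a tuning sound, on AlternativeUse.
; Tick tracks playback time while on, so the channel resumes where it left off.
; Playback shows a delayed track notice from DT_Music, always using the first ChannelsInfo entry.
; Toggling and switching trigger horror event checks, and save events handle power, time and channel state.
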(event `self.BeginLoad`
  ;[1 1 1] On / Off Settings
  (`/Game/HorrorEngine/Blueprints/Core/HorrorEngineMacros.HM_CheckInteraction`)
  (if (`self.On / Off`)
    (`self.PlayRadio`)))

(event `self.Use`
  (params (HorrorEvent :type Boolean))
  ;[1 1 1] Interact Settings
  (`/Game/HorrorEngine/Blueprints/Core/HorrorEngineMacros.HM_CheckInteraction`)
  (if (`self.On / Off`)
    (`self.Close/Off` false)
    (else
      (`self.Open/On` false))))

(event `self.AlternativeUse`
  (params (HorrorEvent :type Boolean))
  ;[1 1 1] Interact Settings
  (`self.SwitchChannel`))

(event `self.Open/On`
  (params (HorrorEvent :type Boolean))
  (bind _on___off (`self.On / Off`))
  (bind _output (`|GetArrayItem` (`self.AddChannels`) (`self.StartChannel`)))
  ;[1 1 1] On / Off Settings
  (`/Game/HorrorEngine/Blueprints/Core/HorrorEngineMacros.HM_CheckInteraction`)
  (if (not (`self.On / Off`))
    (set `self.On / Off` true)
    (`/Game/HorrorEngine/Blueprints/Core/HorrorEngineFunctions.SetMesh` (`self.Radio`) (select `bool` _on___off :`false` (`self.RadioOff`) :`true` (`self.RadioOn`)) :!label _label)
    (`self.HorrorEventCheck` (select `bool` _on___off :`false` "NewEnumerator4" :`true` "NewEnumerator3" :!type "/Game/HorrorEngine/Blueprints/Enums/HorrorEventCheck Enum"))
    (`|ExecutionSequence`
      (:`then_0`
        (set `self.InteractionEnabled` false)
        (bind (_sound _duration) (`/Game/HorrorEngine/Blueprints/Core/HorrorEngineMacros.HM_3DSound` null false (select `bool` (`self.On / Off`) :`false` (`self.TurnOffSound`) :`true` (`self.TurnOnSound`)) (`self.Radio`) (`self.SoundAttenuation`)))
        (`KismetSystemLibrary.Delay` _duration)
        (set `self.InteractionEnabled` true))
      (:`then_1`
        (if (`self.On / Off`)
          (bind (_sound_2 _duration_2) (`/Game/HorrorEngine/Blueprints/Core/HorrorEngineMacros.HM_3DSound` _output false _output (`self.Radio`) (`self.SoundAttenuation`) (`self.CurrentTime`) :!label _label_2))
          (set `self.CurrentDuration` _duration_2)
          (`self.SetActorTickEnabled` true)
          (`KismetSystemLibrary.Delay` 8.0)
          (bind _returnvalue (`|GetDataTableRow` "/Game/EmPath/DataTables/DT_Music.DT_Music" (`|GetArrayItem` (`self.ChannelsInfo`)))
            (:`then`
              (bind _returnvalue_2 (`|CreateWidget` "/Game/EmPath/UI/WB_MusicNotice.WB_MusicNotice_C"))
              (bind (_name _author _music _loop _album) (break `/Game/EmPath/Structures/S_Music` _returnvalue))
              (set `/Game/EmPath/UI/WB_MusicNotice.Album` _album _returnvalue_2)
              (set `/Game/EmPath/UI/WB_MusicNotice.TrackName` _name _returnvalue_2)
              (set `/Game/EmPath/UI/WB_MusicNotice.Author` (`KismetTextLibrary.Conv_StringToText` (`|GetEnumeratorNameAsString` _author)) _returnvalue_2)
              (`UserWidget.AddToViewport` _returnvalue_2 0))
            (:`RowNotFound`
              (bind _returnvalue_3 (`|CreateWidget` "/Game/EmPath/UI/WB_MusicNotice.WB_MusicNotice_C"))
              (set `/Game/EmPath/UI/WB_MusicNotice.Album` "Unknown album" _returnvalue_3)
              (set `/Game/EmPath/UI/WB_MusicNotice.TrackName` "No title" _returnvalue_3)
              (set `/Game/EmPath/UI/WB_MusicNotice.Author` "Unknown artist" _returnvalue_3)
              (`UserWidget.AddToViewport` _returnvalue_3 0)))
          (else
            (`/Game/HorrorEngine/Blueprints/Core/HorrorEngineMacros.HM_Stop3DSound` _output)
            (`/Game/HorrorEngine/Blueprints/Core/HorrorEngineMacros.HM_Stop3DSound` (`self.TuningSound`))
            (`self.SetActorTickEnabled` false)))))))

(event `self.ReceiveTick`
  (params (DeltaSeconds :type "Float (single-precision)"))
  (bind _returnvalue (+ DeltaSeconds (`self.CurrentTime`)))
  ;[1 1 1] Get Playback Time
  (if (not (`self.Switching`))
    (set `self.CurrentTime` (select `bool` (>= _returnvalue (`self.CurrentDuration`)) :`false` _returnvalue))))

(event `self.Close/Off`
  (params (HorrorEvent :type Boolean))
  ;[1 1 1] On / Off Settings
  (`/Game/HorrorEngine/Blueprints/Core/HorrorEngineMacros.HM_CheckInteraction`)
  (if (`self.On / Off`)
    (set `self.On / Off` false)
    (goto _label)))

(event `PlayRadio`
  ;[1 1 1] On / Off Settings
  (goto _label_2))

(event `SwitchChannel`
  (bind _tuningsound (`self.TuningSound`))
  (bind _output (`|GetArrayItem` (`self.AddChannels`) (`self.StartChannel`)))
  ;[1 1 1] Channel Settings
  (if (`self.On / Off`)
    (if (> (`KismetArrayLibrary.Array_LastIndex` (`self.AddChannels`)) 0)
      (set `self.InteractionEnabled` false)
      (set `self.Switching` true)
      (set `self.CurrentTime` 0.0)
      (`/Game/HorrorEngine/Blueprints/Core/HorrorEngineMacros.HM_Stop3DSound` (`|GetArrayItem` (`self.AddChannels`) (`self.StartChannel`)))
      (if (`KismetSystemLibrary.IsValid` (`self.TuningSound`))
        (bind (_sound _duration) (`/Game/HorrorEngine/Blueprints/Core/HorrorEngineMacros.HM_3DSound` _tuningsound false _tuningsound (`self.Radio`) (`self.SoundAttenuation`)))
        (`KismetSystemLibrary.Delay` (- _duration 1.0)))
      (set `self.Switching` false)
      (set `self.InteractionEnabled` true)
      (set `self.StartChannel` (+ (`self.StartChannel`) 1))
      (if (not (`KismetArrayLibrary.Array_IsValidIndex` (`self.AddChannels`) (`self.StartChannel`)))
        (set `self.StartChannel` 0))
      (bind (_sound_2 _duration_2) (`/Game/HorrorEngine/Blueprints/Core/HorrorEngineMacros.HM_3DSound` _output false _output (`self.Radio`) (`self.SoundAttenuation`)))
      (set `self.CurrentDuration` _duration_2)
      (`self.HorrorEventCheck` "NewEnumerator19"))))

(event `self.CollectSaveData`
  ;[0 1 0.5572] Save Settings
  (bind _asmaster (`/Game/HorrorEngine/Blueprints/Core/HorrorEngineFunctions.GetPlayer`))
  (`KismetArrayLibrary.Array_Add` (`/Game/HorrorEngine/Blueprints/Core/HE_SaveGameComponent.AssetCache` (`/Game/HorrorEngine/Blueprints/HorrorEngine.HE_SaveGameComponent` _asmaster)) (make `/Game/HorrorEngine/Blueprints/Structures/SaveStructures/AssetsSave` (`KismetSystemLibrary.GetObjectName` self) (`self.On / Off`) false false false (`self.CurrentTime`) 0.0 (`self.StartChannel`) "+00000000.00:00:00.000000000" "NewEnumerator0" (struct :`Actor` "NewEnumerator0" :`MeshSettings` (struct) :`InspectionSettings` (struct :`InspectionPivotLocation` (0.0 0.0 0.0) :`Takeable` true :`InspectionAnimation` true :`InspectionAnimationSpeedSec` 0.5 :`InspectionBeginRotation` (struct) :`InspectionBeginScale` 1.0 :`MinZoomScale` 1.0 :`MaxZoomScale` 2.0 :`RotationSpeed` 2.5 :`SlideSpeed` 1.0 :`MaxSlideValue` 10.0 :`ItemName` "NSLOCTEXT(\"[E9319CB74B6D000FB1FD816297025122]\", \"B04114684BE13C8CCDB6069E8D44812E\", \"Item Name\")" :`ItemInformation` "NSLOCTEXT(\"[E9319CB74B6D000FB1FD816297025122]\", \"A8A7B76B4C63391D1AC5A7B5D25FB9AE\", \"Item Information\")" :`ReadingText` "NSLOCTEXT(\"[E9319CB74B6D000FB1FD816297025122]\", \"5443C78745510DFFC83277B931F00907\", \"Reading Text\")" :`TakeButton` (struct :`ButtonText` "NSLOCTEXT(\"[E9319CB74B6D000FB1FD816297025122]\", \"9780C15042924951768718B819101440\", \"Take\")") :`ExamineButton` (struct :`ButtonText` "NSLOCTEXT(\"[E9319CB74B6D000FB1FD816297025122]\", \"5175E901487A84D459C6CCAF41D0E6C4\", \"Examine\")") :`ZoomPanButton` (struct :`ButtonText` "NSLOCTEXT(\"[E9319CB74B6D000FB1FD816297025122]\", \"1637EA9C4CEBCB9F6A7CD08E1CBC13F0\", \"Zoom/Slide\")") :`DismissButton` (struct :`ButtonText` "NSLOCTEXT(\"[E9319CB74B6D000FB1FD816297025122]\", \"5A5A20484193E091F4DA148242A59503\", \"Dismiss\")")) :`InventorySettings` (struct :`StorageType` "NewEnumerator3" :`NumberofItemstoAddInventory` 1 :`Interactable` true :`InteractionButton` (struct :`ButtonText` "NSLOCTEXT(\"[E9319CB74B6D000FB1FD816297025122]\", \"97A9B9D546AE5B371A60B2BF356CB282\", \"Use\")") :`SwitchButton` (struct :`ButtonText` "NSLOCTEXT(\"[E9319CB74B6D000FB1FD816297025122]\", \"0D5923514466DE04116E9EA58004B602\", \"Switch\")") :`ZoomSlideButton` (struct :`ButtonText` "NSLOCTEXT(\"[E9319CB74B6D000FB1FD816297025122]\", \"7F750DF3455A9335558F4A9BD1D2A436\", \"Zoom/Slide\")") :`CloseInventoryButton` (struct :`ButtonText` "NSLOCTEXT(\"[E9319CB74B6D000FB1FD816297025122]\", \"2EB73C5B425A32CFA76B8BA90D6BD57D\", \"Close\")")) :`Pistol_MeshSettingsTop` (struct) :`Vhs_CurrentTime` "+00000000.00:00:00.000000000"))))

(event `self.RestoreSaveData`
  (params (AssetSave :type "/Game/HorrorEngine/Blueprints/Structures/SaveStructures/AssetsSave Structure"))
  (bind ((`BooleanSlot01_63_ED79FB5D49E9ED6768D7AE96EDFDE8DB` _booleanslot01) (`BooleanSlot02_64_3DE3E28A45CAE9F3E913659977556562` _booleanslot02) (`BooleanSlot03_65_04AA048C42686C9D2AF003962AEB7F6C` _booleanslot03) (`BooleanSlot04_66_3CB4510F40F5DDD3D81BCEA77398809A` _booleanslot04) (`FloatSlot01_62_3D225DB249A703592AAD5A8405C67C24` _floatslot01) (`FloatSlot02_72_0C6E79544AA699EC0216E1929F2FE1AC` _floatslot02) (`IntegerSlot01_75_ABA8053D4F033D11B1D4ECB38D77F6AB` _integerslot01)) (break `/Game/HorrorEngine/Blueprints/Structures/SaveStructures/AssetsSave` AssetSave))
  ;[0 1 0.5572] Save Settings
  (set `self.On / Off` _booleanslot01)
  (set `self.CurrentTime` _floatslot01)
  (set `self.StartChannel` _integerslot01)
  (`/Game/HorrorEngine/Blueprints/Core/HorrorEngineFunctions.SetMesh` (`self.Radio`) (select `bool` (`self.On / Off`) :`false` (`self.RadioOff`) :`true` (`self.RadioOn`)))
  (if (`self.On / Off`)
    (`self.PlayRadio`)))

(fn `UserConstructionScript`
  (`/Game/HorrorEngine/Blueprints/Core/HorrorEngineMacros.HM_DefaultConstructions` (`self.CreateNewHorrorEvent`))
  (`/Game/HorrorEngine/Blueprints/Core/HorrorEngineFunctions.SetMesh` (`self.Radio`) (select `bool` (`self.On / Off`) :`false` (`self.RadioOff`) :`true` (`self.RadioOn`))))