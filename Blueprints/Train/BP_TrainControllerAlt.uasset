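; Train pawn that follows the first BP_RailRoad spline, with station stops, doors and random pickpocketing.
; Tick drives movement and audio, steering toward a tangent look-ahead point, while a Boost/Brake timeline ramps max speed.
; Station logic brakes, opens one side's doors, then restarts after a delay.
; Between stations, player overlaps toggle door pairs via visibility and collision, sometimes triggering a pickpocket notice; sliding-door animation is unwired.
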(event `self.ReceiveBeginPlay`
  (bind _outactors (`GameplayStatics.GetAllActorsOfClass` "/Game/EmPath/Blueprints/BP_RailRoad.BP_RailRoad_C"))
  (set `self.ActivePath` (`|GetArrayItem` _outactors))
  (`self.Brake`)
  (`KismetSystemLibrary.Delay` 2.0)
  (`self.Boost`))

(event `self.ReceiveTick`
  (params (DeltaSeconds :type "Float (single-precision)"))
  (bind _audio (`self.Audio`))
  (if (`self.Stop`)
    (`AudioComponent.SetVolumeMultiplier` _audio 0.0)
    (else
      (`AudioComponent.SetVolumeMultiplier` _audio 2.0)
      (`self.AddMovementInput` (`self.GetActorForwardVector`) (`self.Speed`))
      (`self.GetPath`))))

(event `self.StartTrain`
  (params (OpenRight :type Boolean) (StationName :type String))
  (`GameplayStatics.PlaySoundAtLocation` "/Game/HorrorEngine/Audio/_ReferenceCues/E-DoorCloseHit_Ref.E-DoorCloseHit_Ref" (0.0 0.0 0.0) (struct) 0.3 1.0 0.0 null "/Game/EmPath/Music/SC_UniqueSound.SC_UniqueSound" null null)
  (set `self.StopAtStation` false)
  (`SceneComponent.SetVisibility` (`self.Left3b`) true false)
  (`SceneComponent.SetVisibility` (`self.Left1b`) true false)
  (`SceneComponent.SetVisibility` (`self.Left2b`) true false)
  (`SceneComponent.SetVisibility` (`self.Left2a`) true false)
  (`SceneComponent.SetVisibility` (`self.Left3a`) true false)
  (`SceneComponent.SetVisibility` (`self.Left1a`) true false)
  (`SceneComponent.SetVisibility` (`self.Right3b`) true false)
  (`SceneComponent.SetVisibility` (`self.Right2b`) true false)
  (`SceneComponent.SetVisibility` (`self.Right3a`) true false)
  (`SceneComponent.SetVisibility` (`self.Right1b`) true false)
  (`SceneComponent.SetVisibility` (`self.Right1a`) true false)
  (`SceneComponent.SetVisibility` (`self.Right2a`) true false)
  (`PrimitiveComponent.SetCollisionEnabled` (`self.Left3b`) "QueryOnly")
  (`PrimitiveComponent.SetCollisionEnabled` (`self.Left1b`) "QueryOnly")
  (`PrimitiveComponent.SetCollisionEnabled` (`self.Left2b`) "QueryOnly")
  (`PrimitiveComponent.SetCollisionEnabled` (`self.Left2a`) "QueryOnly")
  (`PrimitiveComponent.SetCollisionEnabled` (`self.Left3a`) "QueryOnly")
  (`PrimitiveComponent.SetCollisionEnabled` (`self.Left1a`) "QueryOnly")
  (`PrimitiveComponent.SetCollisionEnabled` (`self.Right3b`) "QueryOnly")
  (`PrimitiveComponent.SetCollisionEnabled` (`self.Right3a`) "QueryOnly")
  (`PrimitiveComponent.SetCollisionEnabled` (`self.Right2b`) "QueryOnly")
  (`PrimitiveComponent.SetCollisionEnabled` (`self.Right1b`) "QueryOnly")
  (`PrimitiveComponent.SetCollisionEnabled` (`self.Right2a`) "QueryOnly")
  (`PrimitiveComponent.SetCollisionEnabled` (`self.Right1a`) "QueryOnly")
  (`KismetSystemLibrary.Delay` 2.0)
  (`self.Boost`)
  (goto _label :!via `Reset`))

(event `self.StopTrain`
  (params (OpenRight :type Boolean) (StationName :type String))
  (`/Engine/EditorBlueprintResources/StandardMacros.DoOnce` false :!label _label
    (:`Completed`
      (`self.Brake`)
      (`KismetSystemLibrary.Delay` 5.0)
      (`GameplayStatics.PlaySoundAtLocation` "/Game/HorrorEngine/Audio/Elecronic/E-DoorOpen.E-DoorOpen" (0.0 0.0 0.0) (struct) 0.3 1.0 0.0 null "/Game/EmPath/Music/SC_UniqueSound.SC_UniqueSound" null null)
      (set `self.StopAtStation` true)
      (if OpenRight
        (`SceneComponent.SetVisibility` (`self.Left3b`) false false)
        (`SceneComponent.SetVisibility` (`self.Left1b`) false false)
        (`SceneComponent.SetVisibility` (`self.Left2b`) false false)
        (`SceneComponent.SetVisibility` (`self.Left2a`) false false)
        (`SceneComponent.SetVisibility` (`self.Left3a`) false false)
        (`SceneComponent.SetVisibility` (`self.Left1a`) false false)
        (`PrimitiveComponent.SetCollisionEnabled` (`self.Left3b`) "NoCollision")
        (`PrimitiveComponent.SetCollisionEnabled` (`self.Left1b`) "NoCollision")
        (`PrimitiveComponent.SetCollisionEnabled` (`self.Left2b`) "NoCollision")
        (`PrimitiveComponent.SetCollisionEnabled` (`self.Left2a`) "NoCollision")
        (`PrimitiveComponent.SetCollisionEnabled` (`self.Left3a`) "NoCollision")
        (`PrimitiveComponent.SetCollisionEnabled` (`self.Left1a`) "NoCollision")
        (else
          (`SceneComponent.SetVisibility` (`self.Right3b`) false false)
          (`SceneComponent.SetVisibility` (`self.Right3a`) false false)
          (`SceneComponent.SetVisibility` (`self.Right2b`) false false)
          (`SceneComponent.SetVisibility` (`self.Right2a`) false false)
          (`SceneComponent.SetVisibility` (`self.Right1b`) false false)
          (`SceneComponent.SetVisibility` (`self.Right1a`) false false)
          (`PrimitiveComponent.SetCollisionEnabled` (`self.Right3a`) "NoCollision")
          (`PrimitiveComponent.SetCollisionEnabled` (`self.Right3b`) "NoCollision")
          (`PrimitiveComponent.SetCollisionEnabled` (`self.Right2b`) "NoCollision")
          (`PrimitiveComponent.SetCollisionEnabled` (`self.Right2a`) "NoCollision")
          (`PrimitiveComponent.SetCollisionEnabled` (`self.Right1b`) "NoCollision")
          (`PrimitiveComponent.SetCollisionEnabled` (`self.Right1a`) "NoCollision")))
      (`KismetSystemLibrary.Delay` 8.0)
      (`self.StartTrain` OpenRight))))

(event `self.DoorMiddleRight.OnComponentBeginOverlap`
  (params (OverlappedComponent :type "PrimitiveComponent Object Reference") (OtherActor :type "Actor Object Reference") (OtherComp :type "PrimitiveComponent Object Reference") (OtherBodyIndex :type Integer) (bFromSweep :type Boolean) (SweepResult :type "HitResult Structure (by ref)"))
  (`self.IsPlayer` OtherActor)
  (set `self.LeftDoor` (`self.Left2a`))
  (set `self.RightDoor` (`self.Left2b`))
  (`self.OpenDoor`))

(event `self.Boost`
  (bind (_direction _speed) (`Timeline|Timeline` :!label _label_2)
    (:`Update`
      (bind _output_get (set `FloatingPawnMovement.MaxSpeed` _speed (`self.FloatingPawnMovement`)))
      (set `self.Stop` (< _output_get 0.0)))))

(event `self.Brake`
  (goto _label_2 :!via `Reverse`))

(event `self.DoorMiddleRight.OnComponentEndOverlap`
  (params (OverlappedComponent :type "PrimitiveComponent Object Reference") (OtherActor :type "Actor Object Reference") (OtherComp :type "PrimitiveComponent Object Reference") (OtherBodyIndex :type Integer))
  (`self.IsPlayer` OtherActor)
  (`self.CloseDoor`))

(event `self.FR.OnComponentBeginOverlap`
  (params (OverlappedComponent :type "PrimitiveComponent Object Reference") (OtherActor :type "Actor Object Reference") (OtherComp :type "PrimitiveComponent Object Reference") (OtherBodyIndex :type Integer) (bFromSweep :type Boolean) (SweepResult :type "HitResult Structure (by ref)"))
  (`self.IsPlayer` OtherActor)
  (set `self.LeftDoor` (`self.Right1a`))
  (set `self.RightDoor` (`self.Right1b`))
  (`self.OpenDoor`))

(event `OpenDoor`
  (bind _rightdoor (`self.RightDoor`))
  (bind _leftdoor (`self.LeftDoor`))
  (`GameplayStatics.PlaySoundAtLocation` "/Game/HorrorEngine/Audio/Elecronic/E-DoorOpen.E-DoorOpen" (`SceneComponent.K2_GetComponentLocation` (`self.RightDoor`)) (struct) 0.3 1.0 0.0 null "/Game/EmPath/Music/SC_UniqueSound.SC_UniqueSound" null null)
  (`SceneComponent.SetVisibility` _rightdoor false false)
  (`SceneComponent.SetVisibility` _leftdoor false false)
  (`PrimitiveComponent.SetCollisionEnabled` _rightdoor "NoCollision")
  (`PrimitiveComponent.SetCollisionEnabled` _leftdoor "NoCollision")
  (if (< (`KismetMathLibrary.RandomFloatInRange` 0.0 1.0) 0.3)
    (`KismetSystemLibrary.Delay` 5.0)
    (`self.PickPocket`)))

(event `self.FR.OnComponentEndOverlap`
  (params (OverlappedComponent :type "PrimitiveComponent Object Reference") (OtherActor :type "Actor Object Reference") (OtherComp :type "PrimitiveComponent Object Reference") (OtherBodyIndex :type Integer))
  (`self.IsPlayer` OtherActor)
  (`self.CloseDoor`))

(event `CloseDoor`
  (`GameplayStatics.PlaySoundAtLocation` "/Game/HorrorEngine/Audio/Elecronic/E-DoorCloseHit.E-DoorCloseHit" (`SceneComponent.K2_GetComponentLocation` (`self.RightDoor`)) (struct) 0.3 1.0 0.0 null "/Game/EmPath/Music/SC_UniqueSound.SC_UniqueSound" null null)
  (`SceneComponent.SetVisibility` (`self.RightDoor`) true false)
  (`SceneComponent.SetVisibility` (`self.LeftDoor`) true false)
  (`PrimitiveComponent.SetCollisionEnabled` (`self.LeftDoor`) "QueryOnly")
  (`PrimitiveComponent.SetCollisionEnabled` (`self.RightDoor`) "QueryOnly"))

(event `self.DoorMiddleRight5.OnComponentBeginOverlap`
  (params (OverlappedComponent :type "PrimitiveComponent Object Reference") (OtherActor :type "Actor Object Reference") (OtherComp :type "PrimitiveComponent Object Reference") (OtherBodyIndex :type Integer) (bFromSweep :type Boolean) (SweepResult :type "HitResult Structure (by ref)"))
  (`self.IsPlayer` OtherActor)
  (set `self.LeftDoor` (`self.Right2b`))
  (set `self.RightDoor` (`self.Right2a`))
  (`self.OpenDoor`))

(event `self.DoorMiddleRight5.OnComponentEndOverlap`
  (params (OverlappedComponent :type "PrimitiveComponent Object Reference") (OtherActor :type "Actor Object Reference") (OtherComp :type "PrimitiveComponent Object Reference") (OtherBodyIndex :type Integer))
  (`self.IsPlayer` OtherActor)
  (`self.CloseDoor`))

(event `self.DoorMiddleRight3.OnComponentBeginOverlap`
  (params (OverlappedComponent :type "PrimitiveComponent Object Reference") (OtherActor :type "Actor Object Reference") (OtherComp :type "PrimitiveComponent Object Reference") (OtherBodyIndex :type Integer) (bFromSweep :type Boolean) (SweepResult :type "HitResult Structure (by ref)"))
  (`self.IsPlayer` OtherActor)
  (set `self.LeftDoor` (`self.Left3b`))
  (set `self.RightDoor` (`self.Left3a`))
  (`self.OpenDoor`))

(event `self.DoorMiddleRight3.OnComponentEndOverlap`
  (params (OverlappedComponent :type "PrimitiveComponent Object Reference") (OtherActor :type "Actor Object Reference") (OtherComp :type "PrimitiveComponent Object Reference") (OtherBodyIndex :type Integer))
  (`self.IsPlayer` OtherActor)
  (`self.CloseDoor`))

(event `self.DoorMiddleRight4.OnComponentBeginOverlap`
  (params (OverlappedComponent :type "PrimitiveComponent Object Reference") (OtherActor :type "Actor Object Reference") (OtherComp :type "PrimitiveComponent Object Reference") (OtherBodyIndex :type Integer) (bFromSweep :type Boolean) (SweepResult :type "HitResult Structure (by ref)"))
  (`self.IsPlayer` OtherActor)
  (set `self.LeftDoor` (`self.Right3a`))
  (set `self.RightDoor` (`self.Right3b`))
  (`self.OpenDoor`))

(event `self.DoorMiddleRight4.OnComponentEndOverlap`
  (params (OverlappedComponent :type "PrimitiveComponent Object Reference") (OtherActor :type "Actor Object Reference") (OtherComp :type "PrimitiveComponent Object Reference") (OtherBodyIndex :type Integer))
  (`self.IsPlayer` OtherActor)
  (`self.CloseDoor`))

(event `self.DoorMiddleRight1.OnComponentBeginOverlap`
  (params (OverlappedComponent :type "PrimitiveComponent Object Reference") (OtherActor :type "Actor Object Reference") (OtherComp :type "PrimitiveComponent Object Reference") (OtherBodyIndex :type Integer) (bFromSweep :type Boolean) (SweepResult :type "HitResult Structure (by ref)"))
  (`self.IsPlayer` OtherActor)
  (set `self.LeftDoor` (`self.Left1b`))
  (set `self.RightDoor` (`self.Left1a`))
  (`self.OpenDoor`))

(event `self.DoorMiddleRight1.OnComponentEndOverlap`
  (params (OverlappedComponent :type "PrimitiveComponent Object Reference") (OtherActor :type "Actor Object Reference") (OtherComp :type "PrimitiveComponent Object Reference") (OtherBodyIndex :type Integer))
  (`self.IsPlayer` OtherActor)
  (`self.CloseDoor`))

(fn `GetPath`
  (bind _returnvalue (`self.K2_GetActorLocation`))
  (bind _activepath (`self.ActivePath`))
  (bind _spline (`/Game/EmPath/Blueprints/BP_RailRoad.Spline` _activepath))
  (`/Engine/EditorBlueprintResources/StandardMacros.IsValid` _activepath
    (:`Is Valid`
      (if (== (`SplineComponent.GetLocationAtSplinePoint` _spline (`SplineComponent.GetNumberOfSplinePoints` _spline) "World") _returnvalue :`ErrorTolerance` 50.0)
        (set `self.Stop` true)
        (else
          (`self.K2_SetActorRotation` (`KismetMathLibrary.FindLookAtRotation` _returnvalue (`SplineComponent.FindLocationClosestToWorldLocation` _spline (+ (* (`KismetMathLibrary.Normal` (`SplineComponent.FindTangentClosestToWorldLocation` _spline _returnvalue "World")) 50.0) _returnvalue) "World"))))))))

(fn `PickPocket`
  (`/Game/HorrorEngine/Blueprints/Core/HorrorEngineFunctions.Notice` "You have been pickpocketed!" (`KismetTextLibrary.Conv_StringToText` (`KismetStringLibrary.Concat_StrStr` (`KismetTextLibrary.Conv_TextToString` (`KismetTextLibrary.Conv_IntToText` (`KismetMathLibrary.RandomIntegerInRange` 1 20))) " €")) "lost."))

(fn `UserConstructionScript`)