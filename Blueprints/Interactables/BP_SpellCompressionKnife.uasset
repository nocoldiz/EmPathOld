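; BP_SpellCompressionKnife is a usable interactable that completes a spellcrafting ritual, costing the player health and producing a spellbook.
; On Use, it messages every BI_Spellcrafting actor to activate the killing ground and deals fixed damage to the player pawn.
; A nested pass over those actors requests the stored spell, finishes the ritual and spawns BP_Spellbook at the knife's transform, so damage and spawns repeat per loop iteration.
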(event `/Game/HorrorEngine/Blueprints/Core/Use.Use`
  (params (HorrorEvent :type Boolean))
  (bind _outactors (`GameplayStatics.GetAllActorsWithInterface` "/Game/EmPath/Interfaces/BI_Spellcrafting.BI_Spellcrafting_C"))
  (for _array_element _outactors
    (message `/Game/EmPath/Interfaces/BI_Spellcrafting.ActivateKillingGround` _array_element)
    (message `/Game/EmPath/Interfaces/BPI_Damagable.TakeDamage` (`GameplayStatics.GetPlayerPawn` 0) (make `/Game/EmPath/Structures/S_DamageInfo` 5.0) null)
    (bind _outactors_2 (`GameplayStatics.GetAllActorsWithInterface` "/Game/EmPath/Interfaces/BI_Spellcrafting.BI_Spellcrafting_C"))
    (for _array_element_2 _outactors_2
      (message `/Game/EmPath/Interfaces/BI_Spellcrafting.GetStoredSpell` _array_element_2)
      (message `/Game/EmPath/Interfaces/BI_Spellcrafting.FinishRitual` _array_element_2)
      (`|SpawnActorFromClass` "/Game/EmPath/Blueprints/Objects/BP_Spellbook.BP_Spellbook_C" (`self.GetTransform`) "Undefined" "MultiplyWithRoot" null (struct) "NewEnumerator0" false null "/Game/EmPath/SoundCues/SC_Unpack.SC_Unpack" true false "Spellbook" "Use" null))))

(fn `UserConstructionScript`
  (`parent.UserConstructionScript`))