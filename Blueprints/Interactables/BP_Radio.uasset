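; Interactable radio that cycles through Off, AM, FM and EM modes and tunes between audio stations and static.
; Mode changes reset frequency and volume, while tuning steps the frequency, with decreases blocked below the FM floor in every band.
; While on, Tick crossfades station and noise audio by sampling per-channel float curves at the current frequency.
; Switching Off explicitly mutes only the static, and Tick stops updating the stations.
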(event `/Game/EmPath/Interfaces/BI_Radio.CycleFrequency`
  ;[1 1 1] Comment
  (`GameplayStatics.PlaySound2D` "/Game/HorrorEngine/Audio/Button/ClickButtonOn_Cue.ClickButtonOn_Cue" 1.0 1.0 0.0 null null)
  (switch `/Game/EmPath/Enum/E_Radio` (`self.RadioType`)
    (:`NewEnumerator3`
      (set `self.RadioType` "NewEnumerator0")
      (set `self.Frequency` 520.0)
      (set `self.Volume` 1.0)
      (`TextRenderComponent.K2_SetText` (`self.TextRender`) (`self.AMValue`)))
    (:`NewEnumerator0`
      (set `self.RadioType` "NewEnumerator1")
      (set `self.Frequency` 88.0)
      (set `self.Volume` 1.0)
      (`TextRenderComponent.K2_SetText` (`self.TextRender`) (`self.FMValue`)))
    (:`NewEnumerator1`
      (set `self.RadioType` "NewEnumerator2")
      (set `self.Frequency` 1.0)
      (set `self.Volume` 1.0)
      (`TextRenderComponent.K2_SetText` (`self.TextRender`) (`self.EmValue`)))
    (:`NewEnumerator2`
      (set `self.RadioType` "NewEnumerator3")
      (set `self.Volume` 0.0)
      (`AudioComponent.SetVolumeMultiplier` (`self.Noise`) 0.0)
      (`TextRenderComponent.K2_SetText` (`self.TextRender`) (`self.OffValue`)))))

(event `/Game/EmPath/Interfaces/BI_Radio.SetFrequency`
  (params (Inverse :type Boolean))
  (bind _frequency (`self.Frequency`))
  (if Inverse
    (if (not (< (`self.Frequency`) 88.0))
      (set `self.Frequency` (- _frequency 0.1))
      (`TextRenderComponent.K2_SetText` (`self.TextRender`) (`KismetTextLibrary.Conv_StringToText` (`KismetStringLibrary.Concat_StrStr` (`KismetStringLibrary.Conv_DoubleToString` (`self.Frequency`)) (`|GetEnumeratorNameAsString` (`self.RadioType`)))) :!label _label))
    (else
      (set `self.Frequency` (+ _frequency 0.1))
      (goto _label))))

(event `self.ReceiveTick`
  (params (DeltaSeconds :type "Float (single-precision)"))
  (bind _frequency (`self.Frequency`))
  (bind _fm2 (`self.FM2`))
  (bind _fm3 (`self.FM3`))
  (bind _fm4 (`self.FM4`))
  (bind _fm5 (`self.FM5`))
  (bind _fm6 (`self.FM6`))
  (if (not (`|EnumEquality` (`self.RadioType`) "NewEnumerator3"))
    (`|ExecutionSequence`
      (:`then_0`
        ;[1 1 1] BitCrush Station
        (`/Engine/EditorBlueprintResources/StandardMacros.IsValid` (`self.FM1_BitcrushStation`)
          (:`Is Valid`
            (`AudioComponent.SetVolumeMultiplier` (`self.FM1_BitcrushStation`) (* (`CurveFloat.GetFloatValue` (`self.CurveFM1`) _frequency) (`self.Volume`))))))
      (:`then_1`
        ;[1 1 1] Static
        (`/Engine/EditorBlueprintResources/StandardMacros.IsValid` (`self.Noise`)
          (:`Is Valid`
            (`AudioComponent.SetVolumeMultiplier` (`self.Noise`) (* (`CurveFloat.GetFloatValue` (`self.CurveStatic`) _frequency) (`self.Volume`))))))
      (:`then_2`
        ;[1 1 1] BitCrush Station
        (`/Engine/EditorBlueprintResources/StandardMacros.IsValid` _fm2
          (:`Is Valid`
            (`AudioComponent.SetVolumeMultiplier` _fm2 (* (`CurveFloat.GetFloatValue` (`self.CurveFM2`) _frequency) (`self.Volume`))))))
      (:`then_3`
        ;[1 1 1] BitCrush Station
        (`/Engine/EditorBlueprintResources/StandardMacros.IsValid` _fm4
          (:`Is Valid`
            (`AudioComponent.SetVolumeMultiplier` _fm4 (* (`CurveFloat.GetFloatValue` (`self.CurveFM4`) _frequency) (`self.Volume`))))))
      (:`then_4`
        ;[1 1 1] BitCrush Station
        (`/Engine/EditorBlueprintResources/StandardMacros.IsValid` _fm6
          (:`Is Valid`
            (`AudioComponent.SetVolumeMultiplier` _fm6 (* (`CurveFloat.GetFloatValue` (`self.CurveFM6`) _frequency) (`self.Volume`))))))
      (:`then_5`
        ;[1 1 1] BitCrush Station
        (`/Engine/EditorBlueprintResources/StandardMacros.IsValid` _fm5
          (:`Is Valid`
            (`AudioComponent.SetVolumeMultiplier` _fm5 (* (`CurveFloat.GetFloatValue` (`self.CurveFM5`) _frequency) (`self.Volume`))))))
      (:`then_6`
        ;[1 1 1] BitCrush Station
        (`/Engine/EditorBlueprintResources/StandardMacros.IsValid` _fm3
          (:`Is Valid`
            (`AudioComponent.SetVolumeMultiplier` _fm3 (* (`CurveFloat.GetFloatValue` (`self.CurveFM3`) _frequency) (`self.Volume`)))))))))

(fn `Use`
  (params (HorrorEvent :type Boolean))
  (`parent.Use` HorrorEvent))

(fn `UserConstructionScript`
  (`parent.UserConstructionScript`))