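; Camper controller Blueprint sketching a warp-travel state machine between streamed destination levels, though every event is empty and that logic is disconnected.
; The unwired chains read and set the player pawn's driving mode through messages, using delays, hyperspace sounds and level load/unload for arrival, refueling and departure.
; HideAmbience and ShowAmbience toggle visibility and collision on "Scenery"-tagged actors.
; The remaining functions are mostly getter stubs returning defaults.
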(event `InitialState`
  ;[1 1 1] InitialState
)

(event `self.ReceiveBeginPlay`)

(event `/Game/EmPath/Interfaces/BI_GameActions.NextState`)

(event `Depart`)

(fn `CurrentDestination`
  (returns (Destination :type String))
  (return ""))

(fn `GetActiveActor`
  (returns (Actor :type "Actor Object Reference"))
  (return null))

(fn `GetActorLocation`
  (returns (Location :type "Vector Structure"))
  (return (0.0 0.0 0.0)))

(fn `GetCamperMode`
  (returns (DrivingMode :type "/Game/EmPath/Enum/E_DrivingMode Enum"))
  (return "NewEnumerator0"))

(fn `GetCurrentMP`
  (returns (Mp :type "Float (double-precision)"))
  (return 0.0))

(fn `GetIsSitting`
  (returns (IsSitting :type Boolean))
  (return false))

(fn `GetIsTalking`
  (returns (IsTalking :type Boolean))
  (return false))

(fn `GetKnownSpells`
  (returns (Spells :type "Array of /Game/EmPath/Structures/S_SpellInfo Structure"))
  (return))

(fn `GetMapTile`
  (returns (MapTile :type "Vector2D Structure"))
  (return (0.0 0.0)))

(fn `GetMoney`
  (returns (Money :type "Float (double-precision)"))
  (return 0.0))

(fn `GetSelectedSpell`
  (returns (SpellInfo :type "/Game/EmPath/Structures/S_SpellInfo Structure"))
  (return))

(fn `GetSpawnReaction`
  (returns (Spawned :type Boolean))
  (return false))

(fn `GetSpellbookPage`
  (returns (SpellInfo :type "/Game/EmPath/Structures/S_SpellInfo Structure") (MagicInfo :type "/Game/EmPath/Structures/S_MagicSchools Structure") (GlossaryInfo :type "/Game/EmPath/Structures/S_Glossary Structure") (LastPage :type "/Game/EmPath/Enum/E_PageTypes Enum"))
  (return (struct) (struct) (struct) "NewEnumerator0"))

(fn `GetSpellCollision`
  (returns (IsColliding :type Boolean))
  (return false))

(fn `GetVehicle`
  (returns (Vehicle :type "Actor Object Reference"))
  (return null))

(fn `HideAmbience`
  (bind _outactors (`GameplayStatics.GetAllActorsWithTag` "Scenery"))
  (for _array_element _outactors
    (`self.SetActorHiddenInGame` _array_element true)
    (`self.SetActorEnableCollision` _array_element false)))

(fn `NextDestination`
  (returns (Destination :type String))
  (return ""))

(fn `SetCurrentDestination`
  (returns (Destination :type String))
  (return ""))

(fn `ShowAmbience`
  (bind _outactors (`GameplayStatics.GetAllActorsWithTag` "Scenery"))
  (for _array_element _outactors
    (`self.SetActorHiddenInGame` _array_element false)
    (`self.SetActorEnableCollision` _array_element true)))

(fn `UserConstructionScript`)