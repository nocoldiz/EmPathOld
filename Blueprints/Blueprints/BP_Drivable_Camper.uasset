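; BP_Drivable_Camper is a drivable camper vehicle Blueprint that builds on a parent class and adds handling for a third axle.
; Its Attach Nanite To Skeletal Mesh override calls the parent, then attaches the left and right third-axle wheel components to matching skeletal mesh sockets, keeping world transforms.
; The event graph holds only disabled stubs, and the construction script just calls the parent, so all other behavior is inherited.
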(fn `Attach Nanite To Skeletal Mesh`
  (bind _mesh (`self.Mesh`))
  (`parent.Attach Nanite To Skeletal Mesh`)
  (`SceneComponent.K2_AttachToComponent` (`self.SM_Wheel_Axel3_L`) _mesh "wheel_axel3_l" "KeepWorld" "KeepWorld" "KeepWorld" true)
  (`SceneComponent.K2_AttachToComponent` (`self.SM_Wheel_Axel3_R`) _mesh "wheel_axel3_r" "KeepWorld" "KeepWorld" "KeepWorld" true))

(fn `UserConstructionScript`
  (`parent.UserConstructionScript`))