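; BP_RoadForward is a forward road section with optional bridge, lamp, sidewalk, wall and detail parts.
; Its construction script sets the visibility of each part from a boolean variable, so each placed section can show a different combination.
; One bridge flag drives both the upper and lower bridge components, and every visibility change propagates to child components.
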(fn `UserConstructionScript`
  (locals (SidewalkVisible :type Boolean :default false))
  ;[1 1 1] Show / Hide Bridge Lamps
  (`SceneComponent.SetVisibility` (`self.Lamps`) (`self.LampsVisible`) true)
  (`SceneComponent.SetVisibility` (`self.Bridge Lower`) (`self.BridgeVisible`) true)
  (`SceneComponent.SetVisibility` (`self.Bridge Upper`) (`self.BridgeVisible`) true)
  (`SceneComponent.SetVisibility` (`self.sidewalk`) (`local.SidewalkVisible`) true)
  (`SceneComponent.SetVisibility` (`self.Details`) (`self.DetailsVisible`) true)
  (`SceneComponent.SetVisibility` (`self.straightBrdigeWall`) (`self.WallVisible`) true))