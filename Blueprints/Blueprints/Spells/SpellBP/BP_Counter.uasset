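; BP_Counter is a spell-folder Blueprint that shows one of ten numbered Niagara effects, picked at random.
; Its construction script rolls a Count from zero to nine, switches on it as a string, and stores the matching system in ChoosenParticle.
; That asset is then set on the Particle component with override parameters reset.
; The event graph holds only disabled default events, so all logic runs at construction.
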(fn `UserConstructionScript`
  (locals (ChoosenParticle :type "NiagaraSystem Object Reference"))
  (`parent.UserConstructionScript`)
  (bind _output_get (set `self.Count` (`KismetMathLibrary.RandomIntegerInRange` 0 9)))
  (switch `string` (`KismetStringLibrary.Conv_IntToString` _output_get)
    (:`0`
      (set `local.ChoosenParticle` "/Game/Effects/Letters/NS_0.NS_0"))
    (:`1`
      (set `local.ChoosenParticle` "/Game/Effects/Letters/NS_1.NS_1"))
    (:`2`
      (set `local.ChoosenParticle` "/Game/Effects/Letters/NS_2.NS_2"))
    (:`3`
      (set `local.ChoosenParticle` "/Game/Effects/Letters/NS_3.NS_3"))
    (:`4`
      (set `local.ChoosenParticle` "/Game/Effects/Letters/NS_4.NS_4"))
    (:`5`
      (set `local.ChoosenParticle` "/Game/Effects/Letters/NS_5.NS_5"))
    (:`6`
      (set `local.ChoosenParticle` "/Game/Effects/Letters/NS_6.NS_6"))
    (:`7`
      (set `local.ChoosenParticle` "/Game/Effects/Letters/NS_7.NS_7"))
    (:`8`
      (set `local.ChoosenParticle` "/Game/Effects/Letters/NS_8.NS_8"))
    (:`9`
      (set `local.ChoosenParticle` "/Game/Effects/Letters/NS_9.NS_9")))
  (`NiagaraComponent.SetAsset` (`self.Particle`) (`local.ChoosenParticle`) true))