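; BP_SpellHit is a short-lived effect actor for a spell hit, with configurable sound and particle effects.
; The construction script assigns ParticleFx to its Niagara Particle component.
; On BeginPlay it plays SoundFx at its location with orb attenuation, then destroys itself after the DestroyAfter delay.
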(event `self.ReceiveBeginPlay`
  (`GameplayStatics.PlaySoundAtLocation` (`self.SoundFx`) (`self.K2_GetActorLocation` self) (struct) 1.0 1.0 0.0 "/Game/SuperGrid/TutorialLevel/SoundEffects/Attenuation_Orb.Attenuation_Orb" null null null)
  (`KismetSystemLibrary.Delay` (`self.DestroyAfter`))
  (`self.K2_DestroyActor`))

(fn `UserConstructionScript`
  (`NiagaraComponent.SetAsset` (`self.Particle`) (`self.ParticleFx`) true))