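; Animated spellbook actor that flips through an array of page materials with forward and backward turn animations.
; It links itself to the MultiPageTurn anim blueprint and shows two page pairs through four mesh material slots.
; Forward turns advance the index by two when the animation ends, while backward turns decrement it first; Tick applies pending changes to avoid jumping content.
; An automatic page-turn demo remains but is disconnected.
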(event `self.ReceiveBeginPlay`
  ;[1 1 1] Setup the Anim Blueprint
  (set `self.DoTurnForward` (`self.CanIncPageIndex`))
  (bind _output_get (set `self.NextPageIndex` (`self.PageIndex`)))
  (`self.SetPagematerials` _output_get)
  (bind _asmulti_page_turn_anim_blueprint (cast `/Game/OldAnimatedBooks/AnimBlueprints/MultiPageTurn_AnimBlueprint` (`SkeletalMeshComponent.GetAnimInstance` (`self.Mesh`))))
  (bind _output_get_2 (set `self.AnimInstance` _asmulti_page_turn_anim_blueprint))
  (`/Game/OldAnimatedBooks/AnimBlueprints/MultiPageTurn_AnimBlueprint.SetParent` _output_get_2 self))

(event `/Game/EmPath/Interfaces/BI_SpellBook.GoNextPage`
  ;[1 1 1] Start turn forward animation
  (if (not (`self.CanIncPageIndex`))
    (set `self.PageIndex` 0)
    (set `self.NextPageIndex` 0))
  (`/Game/OldAnimatedBooks/AnimBlueprints/MultiPageTurn_AnimBlueprint.PlayTurnForward` (`self.AnimInstance`)))

(event `/Game/EmPath/Interfaces/BI_SpellBook.GoPreviousPage`
  (bind _animinstance (`self.AnimInstance`))
  ;[1 1 1] Start turn backward animation. To turn backwards we need to increment the page index first and then start the actual animation
  (`self.DecrementPageIndex`)
  (if (`self.CanDecPageIndex`)
    (`/Game/OldAnimatedBooks/AnimBlueprints/MultiPageTurn_AnimBlueprint.PlayTurnBackward` _animinstance)
    (else
      (set `self.PageIndex` 18)
      (set `self.NextPageIndex` 0)
      (`/Game/OldAnimatedBooks/AnimBlueprints/MultiPageTurn_AnimBlueprint.PlayTurnBackward` _animinstance))))

(event `self.ReceiveTick`
  (params (DeltaSeconds :type "Float (single-precision)"))
  (bind _nextpageindex (`self.NextPageIndex`))
  ;[1 1 1] We need to update the page content within one frame to avoid "jumping" page content
  (if (!= (`self.PageIndex`) (`self.NextPageIndex`))
    (`self.SetPagematerials` _nextpageindex)
    (set `self.PageIndex` _nextpageindex)))

(event `PlayTurnReverseEnd`
  ;[1 1 1] Event after turn backwards has finished
)

(event `PlayTurnForwardEnd`
  ;[1 1 1] Increment page index after Turn forward animation has finished
  (`self.IncrementPageIndex`))

(fn `UserConstructionScript`)