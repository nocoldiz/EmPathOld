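; BP_Sword is a melee weapon that damages whatever its Box component overlaps while IsUsing is set.
; Each hit sends blockable, parryable, player-flagged damage by message, plays a sound, spawns blood and prints a debug value.
; If the target's health is then depleted, a random roll can trigger head mutilation through another message.
; An AttackCooldown flag, cleared after AttackDelay, limits repeat hits.
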(event `self.Box.OnComponentBeginOverlap`
  (params (OverlappedComponent :type "PrimitiveComponent Object Reference") (OtherActor :type "Actor Object Reference") (OtherComp :type "PrimitiveComponent Object Reference") (OtherBodyIndex :type Integer) (bFromSweep :type Boolean) (SweepResult :type "HitResult Structure (by ref)"))
  (if (`self.AttackCooldown`)
    _
    (elif (`self.IsUsing`)
      (set `self.AttackCooldown` true)
      (message `/Game/EmPath/Blueprints/DamageSystem/BPI_Damagable.TakeDamage` OtherActor (make `/Game/EmPath/Structures/S_DamageInfo` 30.0 "NewEnumerator1" "NewEnumerator4" false true true false true) null)
      (`GameplayStatics.PlaySoundAtLocation` "/Game/EmPath/Sounds/beheading-sfx-84656.beheading-sfx-84656" (`self.K2_GetActorLocation`) (struct) 1.0 1.0 0.0 null null null null)
      (`GameplayStatics.SpawnEmitterAtLocation` "/Game/Realistic_Starter_VFX_Pack_Vol2/Particles/Blood/P_Blood_Splat_Cone.P_Blood_Splat_Cone" (`self.K2_GetActorLocation` OtherActor))
      (`KismetSystemLibrary.PrintString` (`KismetStringLibrary.Conv_DoubleToString` (`self.ObjectDistance`)))
      ;[1 1 1] Check decapitation
      (if true
        (bind _health (message `/Game/EmPath/Blueprints/DamageSystem/BPI_Damagable.GetCurrentHealth` OtherActor))
        (if (and (<= _health 0.0) (< (`KismetMathLibrary.RandomFloat`) 0.3))
          (message `/Game/EmPath/Blueprints/DamageSystem/BPI_Damagable.Mutilate` OtherActor "Head" false)))
      (`KismetSystemLibrary.Delay` (`self.AttackDelay`))
      (set `self.AttackCooldown` false))))

(fn `UserConstructionScript`
  (`parent.UserConstructionScript`))