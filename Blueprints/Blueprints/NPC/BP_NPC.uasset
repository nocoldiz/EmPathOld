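; BP_NPC is a talkable, shootable sprite-based NPC that yaws toward the player each tick unless turning is disabled.
; Use or TalkEvent calls Talk, which opens a WB_DialogBox with the NPC's lines; repeat calls speed up, then remove it.
; TalkEvent also runs a horror event check.
; Shoot briefly jolts the pivot with random rotation, decrements health and destroys the actor at zero.
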(event `TalkEvent`
  (params (HorrorEvent :type Boolean))
  (`/Game/HorrorEngine/Blueprints/Core/HorrorEngineMacros.HM_CheckInteraction`)
  (`KismetSystemLibrary.PrintString` "HPCello!")
  (`self.HorrorEventCheck` "NewEnumerator0")
  (`self.Talk`))

(event `self.Use`
  (params (HorrorEvent :type Boolean))
  ;[1 1 1] Interact Settings
  (`/Game/HorrorEngine/Blueprints/Core/HorrorEngineMacros.HM_CheckInteraction`)
  (`self.Talk`))

(event `self.ReceiveTick`
  (params (DeltaSeconds :type "Float (single-precision)"))
  ;[1 1 1] Rotate to player
  (if (not (`self.DisableTurn`))
    (bind _location (message `/Game/EmPath/Interfaces/BI_GameActions.GetActorLocation` (`GameplayStatics.GetPlayerPawn` 0)))
    (`self.K2_SetActorRotation` (`KismetMathLibrary.MakeRotator` 0.0 0.0 (.yaw (`KismetMathLibrary.FindLookAtRotation` (`self.K2_GetActorLocation`) _location))))))

(event `self.Shoot`
  (params (HorrorEvent :type Boolean))
  (bind _health (`self.Health`))
  (bind _health_2 (`self.Health`))
  ;[1 1 1] Damage
  (if (not (<= _health 0.0))
    (`SceneComponent.K2_SetRelativeRotation` (`self.NpcPivot`) (`KismetMathLibrary.MakeRotator` (`KismetMathLibrary.RandomFloatInRange` 50.0 20.0) (`KismetMathLibrary.RandomFloatInRange` -20.0 20.0) (`KismetMathLibrary.RandomFloatInRange` -20.0 20.0)) false false)
    (`KismetSystemLibrary.Delay` 0.2)
    (`SceneComponent.K2_SetRelativeRotation` (`self.NpcPivot`) (`KismetMathLibrary.MakeRotator` 0.0) false false)
    (bind _result (`/Engine/EditorBlueprintResources/StandardMacros.DecrementFloat` _health_2)
      (:`  `
        (set `self.Health` _result)
        (`KismetSystemLibrary.PrintString` (`KismetStringLibrary.Conv_DoubleToString` _health))
        (if (<= _health_2 0.0)
          (`self.K2_DestroyActor`))))))

(fn `Talk`
  (bind _widget (`self.Widget`))
  (bind _istalking (message `/Game/EmPath/Interfaces/BI_GameActions.GetIsTalking` (`GameplayStatics.GetPlayerPawn` 0)))
  (if (`self.ShouldRemove`)
    (`/Engine/EditorBlueprintResources/StandardMacros.IsValid` _widget
      (:`Is Valid`
        (`/Game/EmPath/UI/WB_DialogBox.RemoveWidgetNoDelay` _widget)
        (set `self.ShouldRemove` false)))
    (elif _istalking
      (`/Engine/EditorBlueprintResources/StandardMacros.IsValid` _widget
        (:`Is Valid`
          (`/Game/EmPath/UI/WB_DialogBox.SpeedUpDialogue` _widget)
          (set `self.ShouldRemove` true)))
      (else
        (message `/Game/EmPath/Interfaces/BI_GameActions.StartTalking` (`GameplayStatics.GetPlayerPawn` 0) true)
        (bind _returnvalue (`|CreateWidget` "/Game/EmPath/UI/WB_DialogBox.WB_DialogBox_C" null (`self.Pitch`) (`self.Npc Class`) (`self.DialogLines`) (`self.Name_0`)))
        (set `self.Widget` _returnvalue)
        (`UserWidget.AddToViewport` _returnvalue 0)))))

(fn `UserConstructionScript`
  (`/Game/HorrorEngine/Blueprints/Core/HorrorEngineMacros.HM_DefaultConstructions` (`self.CreateNewHorrorEvent`))
  (`/Game/HorrorEngine/Blueprints/Core/HorrorEngineFunctions.SetMesh` (`self.Interact`) (`self.ButtonBaseMesh`))
  (`/Game/HorrorEngine/Blueprints/Core/HorrorEngineFunctions.PlayRate` null (`self.Animation Speed (Sec)`))
  (`PaperFlipbookComponent.SetFlipbook` (`self.Sprite`) (`self.NpcSprite`)))