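; BP_SpellHit is a short-lived effect actor that plays the visual and sound of a spell hit.
; On BeginPlay it sets its particle component to the supplied effect, or to a fixed fire explosion when SpellCharge equals exactly ten.
; It attaches an attenuated, concurrency-limited sound with charge-scaled volume and random pitch.
; After a configurable delay, it starts fading the sound and immediately destroys itself.
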(event `self.ReceiveBeginPlay`
  (if (== (`self.SpellCharge`) 10.0)
    (`NiagaraComponent.SetAsset` (`self.Particle`) "/Game/M5VFXVOL2/Niagara/Explosion/NFire_Exp_00.NFire_Exp_00" true)
    (else
      (`NiagaraComponent.SetAsset` (`self.Particle`) (`self.ParticleFx`) true)))
  (bind _returnvalue (`GameplayStatics.SpawnSoundAttached` (`self.SoundFx`) (`self.Particle`) "None" (0.0 0.0 0.0) (struct) "KeepRelativeOffset" false (* (`self.SpellCharge`) 0.3) (`KismetMathLibrary.RandomFloatInRange` 0.8 1.1) 0.0 "/Game/SuperGrid/TutorialLevel/SoundEffects/Attenuation_Orb.Attenuation_Orb" "/Game/EmPath/Music/SC_SpellConcurrency.SC_SpellConcurrency"))
  (`KismetSystemLibrary.Delay` (`self.DestroyAfter`))
  (`/Engine/EditorBlueprintResources/StandardMacros.IsValid` _returnvalue
    (:`Is Valid`
      (`AudioComponent.FadeOut` _returnvalue 0.6 0.0 "Linear"))
    (:`Is Not Valid`
      _))
  (`self.K2_DestroyActor`))

(fn `UserConstructionScript`
  (locals (NewLocalVar :type "Vector Structure" :default (1.0 1.0 1.0))))