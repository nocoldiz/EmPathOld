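; BP_Counter is a spell Blueprint that rolls a random digit from 0 to 9 whenever its construction script runs.
; The digit, stored as Count, is converted to a string and switched on to set ChoosenParticle, which is applied to the Niagara Particle component with overrides reset.
; Every case assigns None as the particle asset in this graph, and the event graph holds only disabled default events.
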(fn `UserConstructionScript`
  (locals (ChoosenParticle :type "NiagaraSystem Object Reference"))
  (`parent.UserConstructionScript`)
  (bind _output_get (set `self.Count` (`KismetMathLibrary.RandomIntegerInRange` 0 9)))
  (switch `string` (`KismetStringLibrary.Conv_IntToString` _output_get)
    (:`0`
      (set `local.ChoosenParticle` null))
    (:`1`
      (set `local.ChoosenParticle` null))
    (:`2`
      (set `local.ChoosenParticle` null))
    (:`3`
      (set `local.ChoosenParticle` null))
    (:`4`
      (set `local.ChoosenParticle` null))
    (:`5`
      (set `local.ChoosenParticle` null))
    (:`6`
      (set `local.ChoosenParticle` null))
    (:`7`
      (set `local.ChoosenParticle` null))
    (:`8`
      (set `local.ChoosenParticle` null))
    (:`9`
      (set `local.ChoosenParticle` null)))
  (`NiagaraComponent.SetAsset` (`self.Particle`) (`local.ChoosenParticle`) true))