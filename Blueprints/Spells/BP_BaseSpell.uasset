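; Base spell projectile actor, configured by a SpellInfo struct for physics, collision, FX, damage and effects, with a self-target type that skips flight.
; BeginPlay async-loads travel assets and homes enemy casts on the player.
; Impacts route damage and status effects through interfaces, then spawn hit FX, optional actors and AOE damage, with bounce counting before stopping.
; Empty travel, hit, spawn and destroy sequence functions act as hooks.
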(event `self.ReceiveBeginPlay`
  (bind _particle (`self.Particle`))
  (bind (_data _physics _castoptions _travel) (break `/Game/EmPath/Structures/Spell/S_Spell` (`self.SpellInfo`)))
  (bind (_data_2 _physics_2 _castoptions_2 _travel_2 _hit) (break `/Game/EmPath/Structures/Spell/S_Spell` (`self.SpellInfo`)))
  (bind _output (`|ConvertAsset` (`.SoundFx_34_65FD563C4F467E129A41848985070605` (break `/Game/EmPath/Structures/Spell/S_SpellPhase` _travel))))
  ;[1 1 1] Initialize particle FX
  (if (`|EnumEquality` (`.SpellType_10_B7B8C31D4BE12EB0FE170792126AC05D` (break `/Game/EmPath/Structures/Spell/S_SpellData` _data_2)) "NewEnumerator3")
    (`self.TargetSelfPlayer`)
    (else
      (`|LoadAsset` (`.Particle_33_CB2C16674D837A32B01A6EB05D403AC0` (break `/Game/EmPath/Structures/Spell/S_SpellPhase` _travel_2))
        (:`Completed`
          (`|LoadAsset` (`.Particle_33_CB2C16674D837A32B01A6EB05D403AC0` (break `/Game/EmPath/Structures/Spell/S_SpellPhase` _hit))
            (:`Completed`
              (`NiagaraComponent.SetAsset` _particle (`|ConvertAsset` (`.Particle_33_CB2C16674D837A32B01A6EB05D403AC0` (break `/Game/EmPath/Structures/Spell/S_SpellPhase` _travel_2))) true)
              ;[1 1 1 1 28] Set rotation
              (`SceneComponent.SetWorldScale3D` _particle (`.ParticleScale_21_241E48F74D2E3E6A1A39C9A7D27138A9` (break `/Game/EmPath/Structures/Spell/S_SpellPhase` _travel_2)))
              ;[0 1 0.3242] Spell Flowchart
              (`SceneComponent.K2_SetRelativeRotation` (`self.ImpactRadius`) (`KismetMathLibrary.Conv_VectorToRotator` (`self.GetActorForwardVector` (`GameplayStatics.GetPlayerCameraManager` 0))) false false)
              (if (`self.IsCastedByEnemy`)
                (`self.Set Homing Projectile` false))
              (set `self.BounceTimes` (`.BounceTimes_21_21E1EA05490DE4BFF0059B86F1395250` (break `/Game/EmPath/Structures/Spell/S_SpellPhysics` _physics)))
              ;;[1 1 1] Async load particle
              (`|LoadAsset` (`.SoundFx_34_65FD563C4F467E129A41848985070605` (break `/Game/EmPath/Structures/Spell/S_SpellPhase` _travel))
                (:`then`
                  (if (`KismetSystemLibrary.IsValidSoftObjectReference` (`.SpellbookParticles_25_9074207F481940D0E8D947A5B1D5F03F` (break `/Game/EmPath/Structures/Spell/S_SpellCast` _castoptions)))
                    (`|LoadAsset` (`.SpellbookParticles_25_9074207F481940D0E8D947A5B1D5F03F` (break `/Game/EmPath/Structures/Spell/S_SpellCast` _castoptions))
                      (:`then`
                        _)))
                  ;;[1 1 1] Projectile travel
                  (`/Engine/EditorBlueprintResources/StandardMacros.IsValid` _output
                    (:`Is Valid`
                      (bind _returnvalue (`GameplayStatics.SpawnSoundAttached` _output (`self.Particle`) "None" (0.0 0.0 0.0) (struct) "KeepRelativeOffset" true (`self.Volume Multiplier`) (`self.Pitch Multiplier`) 0.0 "/Game/HorrorEngine/Audio/_ATT_Profiles/ATT_Teleport.ATT_Teleport" null))
                      (bind _output_get (set `self.TravelSound` _returnvalue))
                      (if (`self.IsCastedByEnemy`)
                        (if (not (`self.IsHoming`))
                          (`KismetSystemLibrary.Delay` 0.4)
                          (set `ProjectileMovementComponent.bIsHomingProjectile` false (`self.ProjectileMovement`))
                          (`self.PlayTravelSequence` :!label _label)
                          (`KismetSystemLibrary.Delay` (`.DelayBeforeNextPhase_15_31A1C65F4BC3F1626E5972A016AFAF96` (break `/Game/EmPath/Structures/Spell/S_SpellPhase` _travel)))
                          ;;[1 1 1] Destroy sequence
                          (`/Engine/EditorBlueprintResources/StandardMacros.IsValid` _output_get
                            (:`Is Valid`
                              (`AudioComponent.FadeOut` _output_get 1.0 0.0 "Linear"))
                            (:`Is Not Valid`
                              _))
                          (`self.Destroy`))
                        (else
                          (goto _label))))
                    (:`Is Not Valid`
                      (goto _label))))))))))))

(event `StopMovement`
  (bind _travelsound (`self.TravelSound`))
  ;[0 1 0.3242] Spell Flowchart
  ;;[1 1 1] Stop movement
  (`/Engine/EditorBlueprintResources/StandardMacros.IsValid` _travelsound
    (:`Is Valid`
      (`AudioComponent.FadeOut` _travelsound 0.6 0.0 "Linear"))
    (:`Is Not Valid`
      _))
  (`MovementComponent.StopMovementImmediately` (`self.ProjectileMovement`))
  (if (`.DespawnAfterHit_13_3C6F16F14AB50066403B269BB72CECF0` (break `/Game/EmPath/Structures/Spell/S_SpellOptions` (`.Options_30_7158E3F24AB012259CA0A3929FCE79F4` (break `/Game/EmPath/Structures/Spell/S_Spell` (`self.SpellInfo`)))))
    (`self.Destroy`)))

(event `Destroy`
  (bind (_data _physics _castoptions _travel _hit _destroy) (break `/Game/EmPath/Structures/Spell/S_Spell` (`self.SpellInfo`)))
  ;[0 1 0.3242] Spell Flowchart
  ;;[1 1 1] Destroy
  (`self.PlayDestroySequence`)
  (`|LoadAsset` (`.Particle_33_CB2C16674D837A32B01A6EB05D403AC0` (break `/Game/EmPath/Structures/Spell/S_SpellPhase` _destroy))
    (:`then`
      (`|LoadAsset` (`.SoundFx_34_65FD563C4F467E129A41848985070605` (break `/Game/EmPath/Structures/Spell/S_SpellPhase` _destroy))
        (:`then`
          (`|SpawnActorFromClass` "/Game/EmPath/Blueprints/Spells/BP_SpellHit.BP_SpellHit_C" (`KismetMathLibrary.MakeTransform` (`.Location` (`GameplayStatics.BreakHitResult` (`self.Hit`)))) "Undefined" "MultiplyWithRoot" null (`|ConvertAsset` (`.Particle_33_CB2C16674D837A32B01A6EB05D403AC0` (break `/Game/EmPath/Structures/Spell/S_SpellPhase` _destroy))) (`|ConvertAsset` (`.SoundFx_34_65FD563C4F467E129A41848985070605` (break `/Game/EmPath/Structures/Spell/S_SpellPhase` _destroy))) (`.DelayBeforeNextPhase_15_31A1C65F4BC3F1626E5972A016AFAF96` (break `/Game/EmPath/Structures/Spell/S_SpellPhase` _destroy)) (`self.SpellCharge`) null)
          (`self.K2_DestroyActor`))))))

(event `TriggerSpellHit`
  (params (Type :type "/Game/EmPath/Enum/E_SpellImpactTarget Enum" :default "NewEnumerator0"))
  (bind _bouncetimes (`self.BounceTimes`))
  (bind (_data _physics _castoptions _travel _hit) (break `/Game/EmPath/Structures/Spell/S_Spell` (`self.SpellInfo`)))
  (bind (_data_2 _physics_2 _castoptions_2 _travel_2 _hit_2) (break `/Game/EmPath/Structures/Spell/S_Spell` (`self.SpellInfo`)))
  ;[0.9815 0.1329 1] Spell Hit sequence
  ;;[1 1 1] Spell hit events
  (`|LoadAsset` (`.Particle_33_CB2C16674D837A32B01A6EB05D403AC0` (break `/Game/EmPath/Structures/Spell/S_SpellPhase` _hit_2))
    (:`then`
      (`|LoadAsset` (`.SoundFx_34_65FD563C4F467E129A41848985070605` (break `/Game/EmPath/Structures/Spell/S_SpellPhase` _hit_2))
        (:`then`
          (`self.PlayHitSequence`)
          (`|SpawnActorFromClass` "/Game/EmPath/Blueprints/Spells/BP_SpellHit.BP_SpellHit_C" (`KismetMathLibrary.MakeTransform` (`.Location` (`GameplayStatics.BreakHitResult` (`self.Hit`)))) "Undefined" "MultiplyWithRoot" null (`|ConvertAsset` (`.Particle_33_CB2C16674D837A32B01A6EB05D403AC0` (break `/Game/EmPath/Structures/Spell/S_SpellPhase` _hit_2))) (`|ConvertAsset` (`.SoundFx_34_65FD563C4F467E129A41848985070605` (break `/Game/EmPath/Structures/Spell/S_SpellPhase` _hit_2))) (`.DelayBeforeNextPhase_15_31A1C65F4BC3F1626E5972A016AFAF96` (break `/Game/EmPath/Structures/Spell/S_SpellPhase` _hit_2)) (`self.SpellCharge`) null)
          (`|ExecutionSequence`
            (:`then_0`
              (if (`.CanBounce_17_0792C1C9445077127FA70B97E96FD637` (break `/Game/EmPath/Structures/Spell/S_SpellOptions` (`.Options_30_7158E3F24AB012259CA0A3929FCE79F4` (break `/Game/EmPath/Structures/Spell/S_Spell` (`self.SpellInfo`)))))
                ;;[1 1 1] Decrease Max Bounce
                (`/Engine/EditorBlueprintResources/StandardMacros.DecrementInt` _bouncetimes
                  (:`  `
                    (if (== _bouncetimes 0)
                      (`self.StopMovement`))))
                (else
                  (`self.StopMovement`))))
            (:`then_1`
              (if (`KismetSystemLibrary.IsValidSoftClassReference` (`.SpawnActor_36_BBA52AEF4BDEE972254E07B788ACA43B` (break `/Game/EmPath/Structures/Spell/S_SpellPhase` _hit)))
                ;;[1 1 1] SpawnActorOnHit
                (`|LoadAssetClass` (`.SpawnActor_36_BBA52AEF4BDEE972254E07B788ACA43B` (break `/Game/EmPath/Structures/Spell/S_SpellPhase` _hit))
                  (:`then`
                    (if (`.HasCustomSpawnSequence_28_F1D71A79442CAF0723AA38AD074F6EE3` (break `/Game/EmPath/Structures/Spell/S_SpellPhase` _hit))
                      (`self.PlaySpawnSequence`)
                      (else
                        (`|SpawnActorFromClass` (`|ConvertAsset` (`.SpawnActor_36_BBA52AEF4BDEE972254E07B788ACA43B` (break `/Game/EmPath/Structures/Spell/S_SpellPhase` _hit))) (`KismetMathLibrary.Conv_VectorToTransform` (`.ImpactPoint` (`GameplayStatics.BreakHitResult` (`self.Hit`)))) "AdjustIfPossibleButAlwaysSpawn" "MultiplyWithRoot" null null)))))))
            (:`then_2`
              (if (`|EnumEquality` (`.SpellType_10_B7B8C31D4BE12EB0FE170792126AC05D` (break `/Game/EmPath/Structures/Spell/S_SpellData` _data)) "NewEnumerator1")
                (`self.AOEDamage` (`.AOERadius_46_C0EDE6854CC69314A0CA04B7240A4E1E` (break `/Game/EmPath/Structures/Spell/S_SpellData` _data)) (make `/Game/EmPath/Structures/S_DamageInfo` (`.AOEDamage_48_6EF662FB4032989DC133EAB9D11E12B7` (break `/Game/EmPath/Structures/Spell/S_SpellData` _data)) "NewEnumerator3" (`.AOEDamageResponse_51_24BB0BD04069F9338117C9B4A946EC3B` (break `/Game/EmPath/Structures/Spell/S_SpellData` _data)) false false false false true))))
            (:`then_4`
              (switch `/Game/EmPath/Enum/E_SpellImpactTarget` Type))))))))

(event `self.ImpactRadius.OnComponentBeginOverlap`
  (params (OverlappedComponent :type "PrimitiveComponent Object Reference") (OtherActor :type "Actor Object Reference") (OtherComp :type "PrimitiveComponent Object Reference") (OtherBodyIndex :type Integer) (bFromSweep :type Boolean) (SweepResult :type "HitResult Structure (by ref)"))
  ;[1 0.5177 0.03873 1 24] Spell impact
)

(event `TargetSelfPlayer`
  (bind _returnvalue (`GameplayStatics.GetPlayerPawn` 0))
  (bind (_data _physics _castoptions _travel _hit _destroy _options _effect) (break `/Game/EmPath/Structures/Spell/S_Spell` (`self.SpellInfo`)))
  (bind (_duration _magnitude _successrate _enable _effect_2) (break `/Game/EmPath/Structures/Spell/S_SpellEffect` _effect))
  ;[1 0.5177 0.03873 1 24] Spell impact
  ;;[1 1 1] Impact with player
  (if (not (`.DontDamageCaster_11_7F4FC5814DA96A66AB5A899A21F0FEEE` (break `/Game/EmPath/Structures/Spell/S_SpellOptions` _options))) :!label _label_2
    (if (> (`.Damage_31_52F4AABF455580D985AAC3AE08AEA426` (break `/Game/EmPath/Structures/Spell/S_SpellData` _data)) 0.0)
      (message `/Game/EmPath/Interfaces/BPI_Damagable.TakeDamage` _returnvalue (make `/Game/EmPath/Structures/S_DamageInfo` (* (`.Damage_31_52F4AABF455580D985AAC3AE08AEA426` (break `/Game/EmPath/Structures/Spell/S_SpellData` _data)) (`self.SpellCharge`)) "NewEnumerator1" (`.DamageResponse_35_CD9268084CD9DB8F1CCB359CE17A7AFA` (break `/Game/EmPath/Structures/Spell/S_SpellData` _data)) false true true false true) null)
      (`self.TriggerSpellHit` "NewEnumerator0"))
    (message `/Game/EmPath/Interfaces/BPI_Damagable.Apply Effect` _returnvalue _effect_2 _duration _magnitude _enable _successrate "None")))

(event `self.ImpactRadius.OnComponentHit`
  (params (HitComponent :type "PrimitiveComponent Object Reference") (OtherActor :type "Actor Object Reference") (OtherComp :type "PrimitiveComponent Object Reference") (NormalImpulse :type "Vector Structure") (Hit :type "HitResult Structure (by ref)"))
  (bind _returnvalue (`GameplayStatics.GetPlayerPawn` 0))
  (bind _travelsound (`self.TravelSound`))
  (bind (_data _physics _castoptions _travel _hit _destroy _options _effect) (break `/Game/EmPath/Structures/Spell/S_Spell` (`self.SpellInfo`)))
  (bind (_data_2 _physics_2 _castoptions_2 _travel_2 _hit_2 _destroy_2 _options_2 _effect_2) (break `/Game/EmPath/Structures/Spell/S_Spell` (`self.SpellInfo`)))
  (bind (_bblockinghit _binitialoverlap _time _distance _location _impactpoint _normal _impactnormal _physmat _hitactor _hitcomponent _hitbonename) (`GameplayStatics.BreakHitResult` (`self.Hit`)))
  (bind (_duration _magnitude _successrate _enable _effect_3) (break `/Game/EmPath/Structures/Spell/S_SpellEffect` _effect_2))
  ;[1 0.5177 0.03873 1 24] Spell impact
  (`/Engine/EditorBlueprintResources/StandardMacros.IsValid` _travelsound
    (:`Is Valid`
      (`AudioComponent.FadeOut` _travelsound 1.0 0.0 "Linear"))
    (:`Is Not Valid`
      _))
  (set `self.Hit` Hit)
  ;;[1 1 1] Check if hit another spell
  (if (not (`KismetMathLibrary.ClassIsChildOf` (`GameplayStatics.GetObjectClass` OtherActor) "BP_BaseSpell_C"))
    ;;[1 1 1] Impact with player
    (if (`self.ActorHasTag` OtherActor "Player")
      (message `/Game/EmPath/Interfaces/BI_GameActions.HitBySpell` _returnvalue (struct))
      (bind _iscolliding (message `/Game/EmPath/Interfaces/BI_GameActions.GetSpellCollision` _returnvalue))
      (if _iscolliding
        (goto _label_2))
      (else
        ;;[1 1 1] Take Damage
        (if (`KismetSystemLibrary.DoesImplementInterface` OtherActor "/Game/EmPath/Interfaces/BPI_Damagable.BPI_Damagable_C")
          (message `/Game/EmPath/Interfaces/BPI_Damagable.TakeDamage` OtherActor (make `/Game/EmPath/Structures/S_DamageInfo` (* (`.Damage_31_52F4AABF455580D985AAC3AE08AEA426` (break `/Game/EmPath/Structures/Spell/S_SpellData` (`.Data_31_F58FFE3A4CA3B15DEF86A698EF9F7A7B` (break `/Game/EmPath/Structures/Spell/S_Spell` (`self.SpellInfo`))))) (`self.SpellCharge`)) "NewEnumerator1") null)
          (`self.TriggerSpellHit` "NewEnumerator1")
          ;;[1 1 1] ApplyEffectOnEnemy
          (if (< (`.SuccessRate_6_81C200F74F720C3CD752F3B7D3334005` (break `/Game/EmPath/Structures/Spell/S_SpellEffect` _effect)) 1.0)
            (if (<= (`KismetMathLibrary.RandomFloatInRange` 0.0 1.0) (`.SuccessRate_6_81C200F74F720C3CD752F3B7D3334005` (break `/Game/EmPath/Structures/Spell/S_SpellEffect` _effect))) :!label _label_3
              (`KismetSystemLibrary.PrintString` (`KismetStringLibrary.Conv_NameToString` _hitbonename))
              (message `/Game/EmPath/Interfaces/BPI_Damagable.Apply Effect` OtherActor (`.Effect_16_76AC07B2466C6EAD6F36C7B98A6D3A9D` (break `/Game/EmPath/Structures/Spell/S_SpellEffect` _effect)) (break `/Game/EmPath/Structures/Spell/S_SpellEffect` _effect) (`.Magnitude_4_EEDC480041B4562628391DAC0054BC03` (break `/Game/EmPath/Structures/Spell/S_SpellEffect` _effect)) (`.Enable_10_148091A34C6482E7EF4C0584F476106B` (break `/Game/EmPath/Structures/Spell/S_SpellEffect` _effect)) (`.SuccessRate_6_81C200F74F720C3CD752F3B7D3334005` (break `/Game/EmPath/Structures/Spell/S_SpellEffect` _effect)) _hitbonename :!label _label_4))
            (else
              (goto _label_4)))
          (else
            ;;[1 1 1] Set Spell compressor
            (if (`KismetSystemLibrary.DoesImplementInterface` OtherActor "/Game/EmPath/Interfaces/BI_SpellCompressor.BI_SpellCompressor_C")
              (message `/Game/EmPath/Interfaces/BI_SpellCompressor.RegisterSpell` OtherActor (`self.SpellInfo`))
              (set `ProjectileMovementComponent.ProjectileGravityScale` -10.0 (`self.ProjectileMovement`))
              (else
                ;;[1 1 1] Object
                (if (`KismetSystemLibrary.DoesImplementInterface` OtherActor "/Game/EmPath/Interfaces/BI_Object.BI_Object_C")
                  (message `/Game/EmPath/Interfaces/BI_Object.Apply Effect` OtherActor _effect_3 _duration _magnitude _enable _successrate)
                  (else
                    ;;[1 1 1] Check Impact with world
                    (if (`.IgnoreWorld_15_3E4B08474C666A681AD322AB997E9023` (break `/Game/EmPath/Structures/Spell/S_SpellOptions` _options_2))
                      (`self.TriggerSpellHit` "NewEnumerator3")
                      (else
                        (`self.TriggerSpellHit` "NewEnumerator3")))
                    (switch `/Game/EmPath/Enum/E_SpellEffect` (`.Effect_16_76AC07B2466C6EAD6F36C7B98A6D3A9D` (break `/Game/EmPath/Structures/Spell/S_SpellEffect` _effect_2))
                      (:`NewEnumerator24`
                        (`GeometryScriptLibrary_SceneUtilityFunctions.SetComponentMaterialList` OtherComp (`|MakeArray` "/Game/EF_Grounds/Shared/House/Effects/Materials/FlatSurfaces/glass_a_foggy_Mat.glass_a_foggy_Mat" "/Game/EF_Grounds/Shared/House/Effects/Materials/FlatSurfaces/glass_a_foggy_Mat.glass_a_foggy_Mat" "/Game/EF_Grounds/Shared/House/Effects/Materials/FlatSurfaces/glass_a_foggy_Mat.glass_a_foggy_Mat" "/Game/EF_Grounds/Shared/House/Effects/Materials/FlatSurfaces/glass_a_foggy_Mat.glass_a_foggy_Mat" "/Game/EF_Grounds/Shared/House/Effects/Materials/FlatSurfaces/glass_a_foggy_Mat.glass_a_foggy_Mat" :!type "MaterialInterface Object Reference") null)))))))))))))

(event `AOEDamage`
  (params (Radius :type "Float (single-precision)") (DamageInfo :type "/Game/EmPath/Structures/S_DamageInfo Structure"))
  (bind (_data _physics _castoptions _travel _hit _destroy _options) (break `/Game/EmPath/Structures/Spell/S_Spell` (`self.SpellInfo`)))
  ;[1 1 1] AOE Damage
  (bind _returnvalue (`|SpawnActorFromClass` "/Game/EmPath/Enemies/LegacySystem/AOE/BP_SpellAOE.BP_SpellAOE_C" (`KismetMathLibrary.MakeTransform` (`self.K2_GetActorLocation`)) "Undefined" "MultiplyWithRoot" null true (`.DontDamageCaster_11_7F4FC5814DA96A66AB5A899A21F0FEEE` (break `/Game/EmPath/Structures/Spell/S_SpellOptions` _options)) false (`GameplayStatics.GetPlayerPawn` 0)))
  (set `/Game/EmPath/Enemies/LegacySystem/AOE/BP_SpellAOE.Radius` Radius _returnvalue)
  (set `/Game/EmPath/Enemies/LegacySystem/AOE/BP_SpellAOE.DamageInfo` DamageInfo _returnvalue)
  (set `/Game/EmPath/Enemies/LegacySystem/AOE/BP_SpellAOE.Delay` (`.AOEDelay_54_A8AF19F34E52BAFCFFAD07A02177BCA4` (break `/Game/EmPath/Structures/Spell/S_SpellData` _data)) _returnvalue)
  (`/Game/EmPath/Enemies/LegacySystem/AOE/BP_SpellAOE.SpawnAOESphere` _returnvalue))

(event `self.ProjectileMovement.OnProjectileBounce`
  (params (ImpactResult :type "HitResult Structure (by ref)") (ImpactVelocity :type "Vector Structure (by ref)"))
  ;[1 0.5177 0.03873 1 24] Spell impact
)

(event `AOEDamageActor`
  (params (Actor :type "Actor Object Reference"))
  ;[1 1 1] AOE Damage
  (message `/Game/EmPath/Interfaces/BPI_Damagable.TakeDamage` Actor (stale `AOEDamage` DamageInfo) (`self.GetOwner`)))

(event `ApplyEffect`
  ;[1 0.5177 0.03873 1 24] Spell impact
  ;;[1 1 1] ApplyEffectOnEnemy
  (goto _label_3))

(event `Trigger`
  ;[1 0.5177 0.03873 1 24] Spell impact
)

(event `Decapitation`
  ;[1 1 1] Check decapitation
  (bind _health (message `/Game/EmPath/Interfaces/BPI_Damagable.GetCurrentHealth` (stale `self.ImpactRadius.OnComponentHit` OtherActor)))
  (if (<= _health 0.0)
    (message `/Game/EmPath/Interfaces/BPI_Damagable.Mutilate` (stale `self.ImpactRadius.OnComponentHit` OtherActor) (`.HitBoneName` (`GameplayStatics.BreakHitResult` (`self.Hit`))) false)))

(fn `PlayCastSequence`)

(fn `PlayDestroySequence`)

(fn `PlayHitSequence`)

(fn `PlaySpawnSequence`)

(fn `PlayTravelSequence`)

(fn `Set Homing Projectile`
  (params (TargetEnemy :type Boolean))
  (bind _projectilemovement (`self.ProjectileMovement`))
  ;[1 1 1] SetHomingProjectile
  (if TargetEnemy
    (bind _asmaster (`/Game/HorrorEngine/Blueprints/Core/HorrorEngineFunctions.GetPlayer`))
    (bind _lasttarget (`/Game/HorrorEngine/Blueprints/HorrorEngine.LastTarget` _asmaster))
    (`/Engine/EditorBlueprintResources/StandardMacros.IsValid` (`|ConvertAsset` _lasttarget)
      (:`Is Valid`
        (bind _output (`|ConvertAsset` _lasttarget))
        (if (`KismetSystemLibrary.DoesImplementInterface` _output "/Game/EmPath/Interfaces/BPI_Damagable.BPI_Damagable_C")
          (bind _health (message `/Game/EmPath/Interfaces/BPI_Damagable.GetCurrentHealth` _output))
          (if (> _health 0.0)
            (bind _returnvalue (`AddComponent|NODE_AddSceneComponent-3`))
            (set `self.Homing Target Component` _returnvalue)
            (set `ProjectileMovementComponent.HomingTargetComponent` (`self.Homing Target Component`) _projectilemovement :!label _label)
            (set `ProjectileMovementComponent.bIsHomingProjectile` true _projectilemovement)
            (set `ProjectileMovementComponent.HomingAccelerationMagnitude` 15000.0 _projectilemovement)))))
    (else
      (bind _asem_path_player (cast `/Game/EmPath/Blueprints/EmPathPlayer` (`GameplayStatics.GetPlayerCharacter` 0)))
      (bind _returnvalue_2 (`AddComponent|NODE_AddSceneComponent-1` :`self` _asem_path_player))
      (set `self.Homing Target Component` _returnvalue_2)
      (goto _label))))

(fn `SpawnEffect`
  (params (SchoolB :type "/Game/EmPath/Enum/E_MagicSchools Enum" :default "NewEnumerator0"))
  (bind _spawned (message `/Game/EmPath/Interfaces/BI_GameActions.GetSpawnReaction` (`GameplayStatics.GetPlayerPawn` 0)))
  (if (not _spawned)
    (`|SpawnActorFromClass` "/Game/EmPath/Blueprints/Spells/BP_ElementalReaction.BP_ElementalReaction_C" (`KismetMathLibrary.Conv_VectorToTransform` (`self.K2_GetActorLocation` self)) "Undefined" "MultiplyWithRoot" null "NewEnumerator0" (`.MagicSchool_32_B742DA574647EDCD572CCEBFCB1B3FA3` (break `/Game/EmPath/Structures/Spell/S_SpellData` (`.Data_31_F58FFE3A4CA3B15DEF86A698EF9F7A7B` (break `/Game/EmPath/Structures/Spell/S_Spell` (`self.SpellInfo`))))) SchoolB null)
    (message `/Game/EmPath/Interfaces/BI_GameActions.SetSpawnReaction` (`GameplayStatics.GetPlayerPawn` 0) true)))

(fn `UserConstructionScript`
  (bind _projectilemovement (`self.ProjectileMovement`))
  (bind _projectilemovement_2 (`self.ProjectileMovement`))
  (bind (_data _physics) (break `/Game/EmPath/Structures/Spell/S_Spell` (`self.SpellInfo`)))
  (bind (_data_2 _physics_2) (break `/Game/EmPath/Structures/Spell/S_Spell` (`self.SpellInfo`)))
  ;[1 1 1] Get Magic school
  ;[1 1 1] Set projectile movement
  (set `ProjectileMovementComponent.InitialSpeed` (break `/Game/EmPath/Structures/Spell/S_SpellPhysics` _physics_2) _projectilemovement)
  (set `ProjectileMovementComponent.MaxSpeed` (break `/Game/EmPath/Structures/Spell/S_SpellPhysics` _physics_2) _projectilemovement)
  (set `ProjectileMovementComponent.ProjectileGravityScale` (`.GravityScale_10_7DED77654D30DEFA67D300AA19FBCDC7` (break `/Game/EmPath/Structures/Spell/S_SpellPhysics` _physics_2)) _projectilemovement)
  (switch `/Game/EmPath/Enum/E_BounceType` (`.BounceType_25_34238D94428878C1CCD71F8A57A544C1` (break `/Game/EmPath/Structures/Spell/S_SpellPhysics` _physics_2))
    (:`NewEnumerator0`
      (set `ProjectileMovementComponent.Bounciness` 0.0 _projectilemovement_2))
    (:`NewEnumerator1`
      (set `ProjectileMovementComponent.Bounciness` 1.0 _projectilemovement_2))
    (:`NewEnumerator2`
      (set `ProjectileMovementComponent.Bounciness` -6.0 _projectilemovement_2))
    (:`NewEnumerator3`
      (set `ProjectileMovementComponent.Bounciness` 0.5 _projectilemovement_2)))
  (if (`.DrawDebug_57_E15961C54527346E0051A8B98AF5E6CC` (break `/Game/EmPath/Structures/Spell/S_SpellData` (`.Data_31_F58FFE3A4CA3B15DEF86A698EF9F7A7B` (break `/Game/EmPath/Structures/Spell/S_Spell` (`self.SpellInfo`)))))
    (`StaticMeshComponent.SetStaticMesh` (`self.StaticMesh`) "/Engine/EditorMeshes/ArcadeEditorSphere.ArcadeEditorSphere"))
  ;[1 1 1] Override static and pawn collision
  (if (`|EnumEquality` (`.IgnoreCollisions_5_E9BAB3884544792318638CB0291449FA` (break `/Game/EmPath/Structures/Spell/S_SpellPhysics` _physics)) "NewEnumerator3")
    (`PrimitiveComponent.SetCollisionResponseToChannel` (`self.ImpactRadius`) "ECC_WorldDynamic" "ECR_Block")
    (`PrimitiveComponent.SetCollisionResponseToChannel` (`self.ImpactRadius`) "ECC_Pawn" "ECR_Block")
    (else
      (if (`|EnumEquality` (`.IgnoreCollisions_5_E9BAB3884544792318638CB0291449FA` (break `/Game/EmPath/Structures/Spell/S_SpellPhysics` _physics)) "NewEnumerator0")
        (`PrimitiveComponent.SetCollisionResponseToChannel` (`self.ImpactRadius`) "ECC_WorldStatic" "ECR_Ignore"))
      (if (`|EnumEquality` (`.IgnoreCollisions_5_E9BAB3884544792318638CB0291449FA` (break `/Game/EmPath/Structures/Spell/S_SpellPhysics` _physics)) "NewEnumerator1")
        (`PrimitiveComponent.SetCollisionResponseToChannel` (`self.ImpactRadius`) "ECC_Pawn" "ECR_Overlap")))))