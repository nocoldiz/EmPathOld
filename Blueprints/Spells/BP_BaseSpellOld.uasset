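; Base spell projectile (named "Old") driven by a SpellInfo struct that sets movement, particles, collision, damage and effects.
; It launches along the camera's forward vector and destroys itself after its travel duration.
; Hits and overlaps damage players or BPI_Damagable actors, with chance-based status effects and mutilation, while spell-on-spell hits spawn BP_ElementalReaction, gated by a player-held flag.
; Impacts spawn FX and optional actors, then bounce or stop; Play*Sequence hooks are empty.
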(event `TriggerSpellHit`
  (params (Type :type "/Game/EmPath/Enum/E_SpellImpactTarget Enum" :default "NewEnumerator0"))
  (bind _bouncetimes (`self.BounceTimes`))
  (bind (_name _magicschool _spelltype _rating _description _prefix _suffix _author _date _class _icon _attachcastanimation _attachbulletanimation _attachhitanimation _attachexplosionanimation _canbeheld _despawnafterhit _dontdestroy _dontwaitbeforecasting _hasmesh _ignorestaticcollision _ignorepawncollision _hascastanimation _externalcast _hideshadow _subtractmpaftercast _shootonnextpistolshot _recastafterhit _spawnmeshonhit _spawnmeshonexplosion _followcaster _dontdamagecaster _sticky _canfrag _ignoreworld _seektarget _mpcost _chaosfactor _deviation _price _speed _delaybeforecastingagain _gravityscale _castduration _healamount _travelduration _mass _maxtraveldistance _starttraveldelay _destroycastfxdelay _damage _delayhitbox _explosionradius _playerspeedduringcast _dailyuses _spawnmultipleistances _spawnmultipledelay _castoffset _hitboxscale _castsound _castfx _bulletparticlefx _hitsound _hitparticlefx _destroysound _destroyfx _bounceafterhit _maxbouncetimes _castspellonimpact _spawnmeshposition _applymaterialfx _bulletsound _spawnactoronhit) (break `/Game/EmPath/Structures/Spell/S_SpellInfoOLD` (`self.SpellInfo`)))
  ;[1 1 1] Spell hit events
  (`self.PlayHitSequence`)
  (`|SpawnActorFromClass` "/Game/EmPath/Blueprints/Spells/BP_SpellHit.BP_SpellHit_C" (`KismetMathLibrary.MakeTransform` (`.Location` (`GameplayStatics.BreakHitResult` (`self.Hit`)))) "Undefined" "MultiplyWithRoot" null _hitparticlefx _hitsound 1.0 null)
  (`|ExecutionSequence`
    (:`then_0`
      (if (`|EnumEquality` _bounceafterhit "NewEnumerator0")
        (`self.StopMovement`)
        (else
          ;[1 1 1] Decrease Max Bounce
          (`/Engine/EditorBlueprintResources/StandardMacros.DecrementInt` _bouncetimes
            (:`  `
              (if (== _bouncetimes 0)
                (`self.StopMovement`)))))))
    (:`then_1`
      ;[1 1 1] SpawnActorOnHit
      (if (`KismetSystemLibrary.IsValidClass` _spawnactoronhit)
        (`|SpawnActorFromClass` _spawnactoronhit (`self.GetTransform` self) "AdjustIfPossibleButAlwaysSpawn" "MultiplyWithRoot" null null)))
    (:`then_4`
      (switch `/Game/EmPath/Enum/E_SpellImpactTarget` Type))))

(event `self.ImpactRadius.OnComponentBeginOverlap`
  (params (OverlappedComponent :type "PrimitiveComponent Object Reference") (OtherActor :type "Actor Object Reference") (OtherComp :type "PrimitiveComponent Object Reference") (OtherBodyIndex :type Integer) (bFromSweep :type Boolean) (SweepResult :type "HitResult Structure (by ref)"))
  (bind (_name _magicschool _spelltype _rating _description _prefix _suffix _author _date _class _icon _attachcastanimation _attachbulletanimation _attachhitanimation _attachexplosionanimation _canbeheld _despawnafterhit _dontdestroy _dontwaitbeforecasting _hasmesh _ignorestaticcollision _ignorepawncollision _hascastanimation _externalcast _hideshadow _subtractmpaftercast _shootonnextpistolshot _recastafterhit _spawnmeshonhit _spawnmeshonexplosion _followcaster _dontdamagecaster _sticky _canfrag _ignoreworld _seektarget _mpcost _chaosfactor _deviation _price _speed _delaybeforecastingagain _gravityscale _castduration _healamount _travelduration _mass _maxtraveldistance _starttraveldelay _destroycastfxdelay _damage _delayhitbox _explosionradius _playerspeedduringcast _dailyuses _spawnmultipleistances _spawnmultipledelay _castoffset _hitboxscale _castsound _castfx _bulletparticlefx _hitsound _hitparticlefx _destroysound _destroyfx _bounceafterhit _maxbouncetimes _castspellonimpact _spawnmeshposition _applymaterialfx _bulletsound _spawnactoronhit _spawnactorondestroy _particlescale _damageresponse) (break `/Game/EmPath/Structures/Spell/S_SpellInfoOLD` (`self.SpellInfo`)))
  ;[1 0.179 0.6676 1 24] Spell impact
  (if (`KismetSystemLibrary.DoesImplementInterface` OtherActor "/Game/EmPath/Blueprints/DamageSystem/BPI_Damagable.BPI_Damagable_C")
    (message `/Game/EmPath/Blueprints/DamageSystem/BPI_Damagable.TakeDamage` OtherActor (make `/Game/EmPath/Structures/S_DamageInfo` _damage "NewEnumerator1" _damageresponse) null)
    (message `/Game/EmPath/Blueprints/DamageSystem/BPI_Damagable.Mutilate` OtherActor "None" true)))

(event `self.ImpactRadius.OnComponentHit`
  (params (HitComponent :type "PrimitiveComponent Object Reference") (OtherActor :type "Actor Object Reference") (OtherComp :type "PrimitiveComponent Object Reference") (NormalImpulse :type "Vector Structure") (Hit :type "HitResult Structure (by ref)"))
  (bind (_bblockinghit _binitialoverlap _time _distance _location _impactpoint _normal _impactnormal _physmat _hitactor _hitcomponent _hitbonename) (`GameplayStatics.BreakHitResult` Hit))
  (bind _returnvalue (`GameplayStatics.GetPlayerPawn` 0))
  (bind (_name _magicschool _spelltype _rating _description _prefix _suffix _author _date _class _icon _attachcastanimation _attachbulletanimation _attachhitanimation _attachexplosionanimation _canbeheld _despawnafterhit _dontdestroy _dontwaitbeforecasting _hasmesh _ignorestaticcollision _ignorepawncollision _hascastanimation _externalcast _hideshadow _subtractmpaftercast _shootonnextpistolshot _recastafterhit _spawnmeshonhit _spawnmeshonexplosion _followcaster _dontdamagecaster _sticky _canfrag _ignoreworld _seektarget _mpcost _chaosfactor _deviation _price _speed _delaybeforecastingagain _gravityscale _castduration _healamount _travelduration _mass _maxtraveldistance _starttraveldelay _destroycastfxdelay _damage _delayhitbox _explosionradius _playerspeedduringcast _dailyuses _spawnmultipleistances _spawnmultipledelay _castoffset _hitboxscale _castsound _castfx _bulletparticlefx _hitsound _hitparticlefx _destroysound _destroyfx _bounceafterhit _maxbouncetimes _castspellonimpact _spawnmeshposition _applymaterialfx _bulletsound _spawnactoronhit _spawnactorondestroy _particlescale _damageresponse) (break `/Game/EmPath/Structures/Spell/S_SpellInfoOLD` (`self.SpellInfo`)))
  (bind (_name_2 _magicschool_2 _spelltype_2 _rating_2 _description_2 _prefix_2 _suffix_2 _author_2 _date_2 _class_2 _icon_2 _attachcastanimation_2 _attachbulletanimation_2 _attachhitanimation_2 _attachexplosionanimation_2 _canbeheld_2 _despawnafterhit_2 _dontdestroy_2 _dontwaitbeforecasting_2 _hasmesh_2 _ignorestaticcollision_2 _ignorepawncollision_2 _hascastanimation_2 _externalcast_2 _hideshadow_2 _subtractmpaftercast_2 _shootonnextpistolshot_2 _recastafterhit_2 _spawnmeshonhit_2 _spawnmeshonexplosion_2 _followcaster_2 _dontdamagecaster_2 _sticky_2 _canfrag_2 _ignoreworld_2 _seektarget_2 _mpcost_2 _chaosfactor_2 _deviation_2 _price_2 _speed_2 _delaybeforecastingagain_2 _gravityscale_2 _castduration_2 _healamount_2 _travelduration_2 _mass_2 _maxtraveldistance_2 _starttraveldelay_2 _destroycastfxdelay_2 _damage_2 _delayhitbox_2 _explosionradius_2 _playerspeedduringcast_2 _dailyuses_2 _spawnmultipleistances_2 _spawnmultipledelay_2 _castoffset_2 _hitboxscale_2 _castsound_2 _castfx_2 _bulletparticlefx_2 _hitsound_2 _hitparticlefx_2 _destroysound_2 _destroyfx_2 _bounceafterhit_2 _maxbouncetimes_2 _castspellonimpact_2 _spawnmeshposition_2 _applymaterialfx_2 _bulletsound_2 _spawnactoronhit_2 _spawnactorondestroy_2 _particlescale_2 _damageresponse_2 _spelleffect _effectmagnitude _effectduration _effectenable _effectsuccesrate) (break `/Game/EmPath/Structures/Spell/S_SpellInfoOLD` (`self.SpellInfo`)))
  (bind (_name_3 _magicschool_3 _spelltype_3 _rating_3 _description_3 _prefix_3 _suffix_3 _author_3 _date_3 _class_3 _icon_3 _attachcastanimation_3 _attachbulletanimation_3 _attachhitanimation_3 _attachexplosionanimation_3 _canbeheld_3 _despawnafterhit_3 _dontdestroy_3 _dontwaitbeforecasting_3 _hasmesh_3 _ignorestaticcollision_3 _ignorepawncollision_3 _hascastanimation_3 _externalcast_3 _hideshadow_3 _subtractmpaftercast_3 _shootonnextpistolshot_3 _recastafterhit_3 _spawnmeshonhit_3 _spawnmeshonexplosion_3 _followcaster_3 _dontdamagecaster_3 _sticky_3 _canfrag_3 _ignoreworld_3 _seektarget_3 _mpcost_3 _chaosfactor_3 _deviation_3 _price_3 _speed_3 _delaybeforecastingagain_3 _gravityscale_3 _castduration_3 _healamount_3 _travelduration_3 _mass_3 _maxtraveldistance_3 _starttraveldelay_3 _destroycastfxdelay_3 _damage_3 _delayhitbox_3 _explosionradius_3 _playerspeedduringcast_3 _dailyuses_3 _spawnmultipleistances_3 _spawnmultipledelay_3 _castoffset_3 _hitboxscale_3 _castsound_3 _castfx_3 _bulletparticlefx_3 _hitsound_3 _hitparticlefx_3 _destroysound_3 _destroyfx_3 _bounceafterhit_3 _maxbouncetimes_3 _castspellonimpact_3 _spawnmeshposition_3 _applymaterialfx_3 _bulletsound_3 _spawnactoronhit_3 _spawnactorondestroy_3 _particlescale_3 _damageresponse_3 _spelleffect_2) (break `/Game/EmPath/Structures/Spell/S_SpellInfoOLD` (`self.SpellInfo`)))
  (bind (_name_4 _magicschool_4 _spelltype_4 _rating_4 _description_4 _prefix_4 _suffix_4 _author_4 _date_4 _class_4 _icon_4 _attachcastanimation_4 _attachbulletanimation_4 _attachhitanimation_4 _attachexplosionanimation_4 _canbeheld_4 _despawnafterhit_4 _dontdestroy_4 _dontwaitbeforecasting_4 _hasmesh_4 _ignorestaticcollision_4 _ignorepawncollision_4 _hascastanimation_4 _externalcast_4 _hideshadow_4 _subtractmpaftercast_4 _shootonnextpistolshot_4 _recastafterhit_4 _spawnmeshonhit_4 _spawnmeshonexplosion_4 _followcaster_4 _dontdamagecaster_4 _sticky_4 _canfrag_4 _ignoreworld_4 _seektarget_4 _mpcost_4 _chaosfactor_4 _deviation_4 _price_4 _speed_4 _delaybeforecastingagain_4 _gravityscale_4 _castduration_4 _healamount_4 _travelduration_4 _mass_4 _maxtraveldistance_4 _starttraveldelay_4 _destroycastfxdelay_4 _damage_4 _delayhitbox_4 _explosionradius_4 _playerspeedduringcast_4 _dailyuses_4 _spawnmultipleistances_4 _spawnmultipledelay_4 _castoffset_4 _hitboxscale_4 _castsound_4 _castfx_4 _bulletparticlefx_4 _hitsound_4 _hitparticlefx_4 _destroysound_4 _destroyfx_4 _bounceafterhit_4 _maxbouncetimes_4 _castspellonimpact_4 _spawnmeshposition_4 _applymaterialfx_4 _bulletsound_4 _spawnactoronhit_4 _spawnactorondestroy_4 _particlescale_4 _damageresponse_4) (break `/Game/EmPath/Structures/Spell/S_SpellInfoOLD` (`self.SpellInfo`)))
  ;[1 0.179 0.6676 1 24] Spell impact
  (set `self.Hit` Hit)
  ;;[1 1 1] Check if hit another spell
  (`|ExecutionSequence`
    (:`then_0`
      (if (`KismetMathLibrary.ClassIsChildOf` (`GameplayStatics.GetObjectClass` OtherActor) "/Game/EmPath/Blueprints/Spells/BP_BaseSpell.BP_BaseSpell_C")
        ;;[1 1 1] Spell hit Spell
        (`self.SpawnEffect` "NewEnumerator0")
        (`KismetSystemLibrary.Delay` 0.5)
        (message `/Game/EmPath/Interfaces/BI_GameActions.SetSpawnReaction` (`GameplayStatics.GetPlayerCharacter` 0) false)
        (`self.TriggerSpellHit` "NewEnumerator4")
        (else
          ;;[1 1 1] Impact with player
          (if (`self.ActorHasTag` OtherActor "Player")
            (message `/Game/EmPath/Interfaces/BI_GameActions.HitBySpell` _returnvalue (struct))
            (bind _iscolliding (message `/Game/EmPath/Interfaces/BI_GameActions.GetSpellCollision` _returnvalue))
            (if (not _dontdamagecaster)
              (message `/Game/EmPath/Blueprints/DamageSystem/BPI_Damagable.TakeDamage` (`GameplayStatics.GetPlayerPawn` 0) (make `/Game/EmPath/Structures/S_DamageInfo` _damage "NewEnumerator1" _damageresponse false true true false true) null)
              (`self.TriggerSpellHit` "NewEnumerator0"))
            (else
              ;;[1 1 1] Check if hit Damageable Actor
              (if (`KismetSystemLibrary.DoesImplementInterface` OtherActor "/Game/EmPath/Blueprints/DamageSystem/BPI_Damagable.BPI_Damagable_C")
                (message `/Game/EmPath/Blueprints/DamageSystem/BPI_Damagable.TakeDamage` OtherActor (make `/Game/EmPath/Structures/S_DamageInfo` _damage_4 "NewEnumerator1" _damageresponse_4) null)
                (`self.TriggerSpellHit` "NewEnumerator1")
                (`|ExecutionSequence`
                  (:`then_0`
                    ;;[1 1 1] Check decapitation
                    (if _canfrag_3
                      (bind _health (message `/Game/EmPath/Blueprints/DamageSystem/BPI_Damagable.GetCurrentHealth` OtherActor))
                      (if (<= _health 0.0)
                        (message `/Game/EmPath/Blueprints/DamageSystem/BPI_Damagable.Mutilate` OtherActor (`.HitBoneName` (`GameplayStatics.BreakHitResult` (`self.Hit`))) (`|EnumEquality` _spelleffect_2 "NewEnumerator13")))))
                  (:`then_1`
                    ;;[1 1 1] ApplyEffect
                    (if (`|EnumInequality` _spelleffect "NewEnumerator12")
                      (if (<= (`KismetMathLibrary.RandomFloatInRange` 0.0 1.0) _effectsuccesrate) :!label _label
                        (message `/Game/EmPath/Blueprints/DamageSystem/BPI_Damagable.Apply Effect` OtherActor _spelleffect _effectduration _effectmagnitude _effectenable _effectsuccesrate)))))
                (else
                  ;;[1 1 1] Check Impact with world
                  (if (`.IgnoreWorld_257_3428F07E4054AC62823FD2969C3C7CC4` (break `/Game/EmPath/Structures/Spell/S_SpellInfoOLD` (`self.SpellInfo`)))
                    (`self.TriggerSpellHit` "NewEnumerator3")
                    (else
                      (`self.TriggerSpellHit` "NewEnumerator3"))))))))))
    (:`then_1`
      (`KismetSystemLibrary.PrintString` (`KismetStringLibrary.Conv_NameToString` _hitbonename) true true (struct :`G` 0.66 :`B` 1.0 :`A` 1.0) 2.0 _hitbonename))))

(event `ApplyEffect`
  ;[1 0.179 0.6676 1 24] Spell impact
  ;;[1 1 1] ApplyEffect
  (goto _label))

(event `Trigger`
  ;[1 0.179 0.6676 1 24] Spell impact
)

(event `self.ReceiveBeginPlay`
  (bind (_name _magicschool _spelltype _rating _description _prefix _suffix _author _date _class _icon _attachcastanimation _attachbulletanimation _attachhitanimation _attachexplosionanimation _canbeheld _despawnafterhit _dontdestroy _dontwaitbeforecasting _hasmesh _ignorestaticcollision _ignorepawncollision _hascastanimation _externalcast _hideshadow _subtractmpaftercast _shootonnextpistolshot _recastafterhit _spawnmeshonhit _spawnmeshonexplosion _followcaster _dontdamagecaster _sticky _canfrag _ignoreworld _seektarget _mpcost _chaosfactor _deviation _price _speed _delaybeforecastingagain _gravityscale _castduration _healamount _travelduration _mass _maxtraveldistance _starttraveldelay _destroycastfxdelay _damage _delayhitbox _explosionradius _playerspeedduringcast _dailyuses _spawnmultipleistances _spawnmultipledelay _castoffset _hitboxscale _castsound _castfx _bulletparticlefx _hitsound _hitparticlefx _destroysound _destroyfx _bounceafterhit _maxbouncetimes _castspellonimpact _spawnmeshposition _applymaterialfx _bulletsound) (break `/Game/EmPath/Structures/Spell/S_SpellInfoOLD` (`self.SpellInfo`)))
  ;[1 1 1] Set rotation
  (`SceneComponent.K2_SetRelativeRotation` (`self.ImpactRadius`) (`KismetMathLibrary.Conv_VectorToRotator` (`self.GetActorForwardVector` (`GameplayStatics.GetPlayerCameraManager` 0))) false false)
  ;[1 1 1] Projectile travel
  (set `self.BounceTimes` _maxbouncetimes)
  (`GameplayStatics.SpawnSoundAttached` _bulletsound (`self.Particle`) "None" (0.0 0.0 0.0) (struct) "KeepRelativeOffset" false 1.0 1.0 0.0 "/Game/HorrorEngine/Audio/_ATT_Profiles/ATT_Teleport.ATT_Teleport" null)
  (`self.PlayTravelSequence`)
  (`KismetSystemLibrary.Delay` _travelduration)
  ;[1 1 1] Destroy sequence
  (`self.Destroy`))

(event `StopMovement`
  ;[1 1 1] Stop movement
  (`MovementComponent.StopMovementImmediately` (`self.ProjectileMovement`))
  (if (`.DespawnAfterHit_94_FCC803BB45DFD2EBB8E279AC81C92767` (break `/Game/EmPath/Structures/Spell/S_SpellInfoOLD` (`self.SpellInfo`)))
    (`self.Destroy`)))

(event `Destroy`
  (bind (_name _magicschool _spelltype _rating _description _prefix _suffix _author _date _class _icon _attachcastanimation _attachbulletanimation _attachhitanimation _attachexplosionanimation _canbeheld _despawnafterhit _dontdestroy _dontwaitbeforecasting _hasmesh _ignorestaticcollision _ignorepawncollision _hascastanimation _externalcast _hideshadow _subtractmpaftercast _shootonnextpistolshot _recastafterhit _spawnmeshonhit _spawnmeshonexplosion _followcaster _dontdamagecaster _sticky _canfrag _ignoreworld _seektarget _mpcost _chaosfactor _deviation _price _speed _delaybeforecastingagain _gravityscale _castduration _healamount _travelduration _mass _maxtraveldistance _starttraveldelay _destroycastfxdelay _damage _delayhitbox _explosionradius _playerspeedduringcast _dailyuses _spawnmultipleistances _spawnmultipledelay _castoffset _hitboxscale _castsound _castfx _bulletparticlefx _hitsound _hitparticlefx _destroysound _destroyfx _bounceafterhit _maxbouncetimes _castspellonimpact _spawnmeshposition _applymaterialfx _bulletsound _spawnactoronhit _spawnactorondestroy) (break `/Game/EmPath/Structures/Spell/S_SpellInfoOLD` (`self.SpellInfo`)))
  ;[1 1 1] Destroy
  (`self.PlayDestroySequence`)
  (`|SpawnActorFromClass` "/Game/EmPath/Blueprints/Spells/BP_SpellHit.BP_SpellHit_C" (`KismetMathLibrary.MakeTransform` (`.Location` (`GameplayStatics.BreakHitResult` (`self.Hit`)))) "Undefined" "MultiplyWithRoot" null _destroyfx _destroysound 1.0 null)
  ;[1 1 1] SpawnActorOnHit
  (`|SpawnActorFromClass` _spawnactorondestroy (`self.GetTransform` self) "Undefined" "MultiplyWithRoot" null null)
  (`self.K2_DestroyActor`))

(fn `PlayCastSequence`)

(fn `PlayDestroySequence`)

(fn `PlayHitSequence`)

(fn `PlayTravelSequence`)

(fn `SpawnEffect`
  (params (SchoolB :type "/Game/EmPath/Enum/E_MagicSchools Enum" :default "NewEnumerator0"))
  (bind _spawned (message `/Game/EmPath/Interfaces/BI_GameActions.GetSpawnReaction` (`GameplayStatics.GetPlayerPawn` 0)))
  (if (not _spawned)
    (`|SpawnActorFromClass` "/Game/EmPath/Blueprints/Spells/BP_ElementalReaction.BP_ElementalReaction_C" (`KismetMathLibrary.Conv_VectorToTransform` (`self.K2_GetActorLocation` self)) "Undefined" "MultiplyWithRoot" null "NewEnumerator0" (`.MagicSchool_110_2E089C5E42E66A72571EC49C4EAD977D` (break `/Game/EmPath/Structures/Spell/S_SpellInfoOLD` (`self.SpellInfo`))) SchoolB null)
    (message `/Game/EmPath/Interfaces/BI_GameActions.SetSpawnReaction` (`GameplayStatics.GetPlayerPawn` 0) true)))

(fn `UserConstructionScript`
  (bind _projectilemovement (`self.ProjectileMovement`))
  (bind _particle (`self.Particle`))
  (bind (_name _magicschool _spelltype _rating _description _prefix _suffix _author _date _class _icon _attachcastanimation _attachbulletanimation _attachhitanimation _attachexplosionanimation _canbeheld _despawnafterhit _dontdestroy _dontwaitbeforecasting _hasmesh _ignorestaticcollision _ignorepawncollision _hascastanimation _externalcast _hideshadow _subtractmpaftercast _shootonnextpistolshot _recastafterhit _spawnmeshonhit _spawnmeshonexplosion _followcaster _dontdamagecaster _sticky _canfrag _ignoreworld _seektarget _mpcost _chaosfactor _deviation _price _speed _delaybeforecastingagain _gravityscale _castduration _healamount _travelduration _mass _maxtraveldistance _starttraveldelay _destroycastfxdelay _damage _delayhitbox _explosionradius _playerspeedduringcast _dailyuses _spawnmultipleistances _spawnmultipledelay _castoffset _hitboxscale _castsound _castfx _bulletparticlefx _hitsound _hitparticlefx _destroysound _destroyfx _bounceafterhit _maxbouncetimes _castspellonimpact _spawnmeshposition _applymaterialfx _bulletsound _spawnactoronhit _spawnactorondestroy _particlescale) (break `/Game/EmPath/Structures/Spell/S_SpellInfoOLD` (`self.SpellInfo`)))
  ;[1 1 1] Get Magic school
  (bind _returnvalue (`|GetDataTableRow` "/Game/EmPath/DataTables/DT_MagicSchools.DT_MagicSchools" (`KismetStringLibrary.Conv_StringToName` (`|GetEnumeratorNameAsString` (`.MagicSchool_110_2E089C5E42E66A72571EC49C4EAD977D` (break `/Game/EmPath/Structures/Spell/S_SpellInfoOLD` (`self.SpellInfo`))))))
    (:`then`
      (bind _output_get (set `self.MagicSchool` _returnvalue)))
    (:`RowNotFound`
      _))
  ;[1 1 1] Set projectile movement
  (set `ProjectileMovementComponent.InitialSpeed` _speed _projectilemovement)
  (set `ProjectileMovementComponent.MaxSpeed` _speed _projectilemovement)
  (set `ProjectileMovementComponent.ProjectileGravityScale` _gravityscale _projectilemovement)
  ;[1 1 1] Initialize particle FX
  (`/Engine/EditorBlueprintResources/StandardMacros.IsValid` _bulletparticlefx
    (:`Is Valid`
      (`NiagaraComponent.SetAsset` _particle _bulletparticlefx true)
      (`SceneComponent.SetWorldScale3D` _particle (`KismetMathLibrary.Conv_DoubleToVector` _particlescale))
      ;[1 1 1] Override static and pawn collision
      (if _ignorestaticcollision
        (`PrimitiveComponent.SetCollisionResponseToChannel` (`self.ImpactRadius`) "ECC_WorldStatic" "ECR_Ignore"))
      (if _ignorepawncollision
        (`PrimitiveComponent.SetCollisionResponseToChannel` (`self.ImpactRadius`) "ECC_Pawn" "ECR_Overlap")))))