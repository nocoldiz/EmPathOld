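; BP_GenericDoor is a door that responds to status effects by opening or closing.
; ApplyEffect switches on the incoming status: Open Door calls OpenDoor and prints a debug string, while Close Door calls CloseDoor without locking.
; The health, team, damage and attack-token functions are stubs returning zero or false, and construction only runs the parent script.
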(event `/Game/EmPath/Interfaces/BPI_Damagable.Apply Effect`
  (params (Status :type "/Game/EmPath/Enum/E_SpellEffect Enum" :default "NewEnumerator12") (Duration :type "Float (double-precision)") (Magnitude :type "Float (double-precision)") (Enable :type Boolean) (SuccessRate :type "Float (double-precision)"))
  (switch `/Game/EmPath/Enum/E_SpellEffect` Status
    (:`NewEnumerator2`
      (`self.OpenDoor`)
      (`KismetSystemLibrary.PrintString` "Door"))
    (:`NewEnumerator10`
      (`self.CloseDoor` false))))

(fn `GetCurrentHealth`
  (returns (Health :type "Float (double-precision)"))
  (return 0.0))

(fn `GetMaxHealth`
  (returns (MaxHealth :type "Float (double-precision)"))
  (return 0.0))

(fn `GetTeamNumber`
  (returns (TeamNumber :type Integer))
  (return 0))

(fn `Heal`
  (params (Amount :type "Float (double-precision)"))
  (returns (NewHealth :type "Float (double-precision)"))
  (return 0.0))

(fn `IsAttacking`
  (returns (Attacking :type Boolean))
  (return false))

(fn `IsDead`
  (returns (Dead :type Boolean))
  (return false))

(fn `ReserveAttackToken`
  (params (Amount :type Integer))
  (returns (Success :type Boolean))
  (return false))

(fn `TakeDamage`
  (params (DamageInfo :type "/Game/EmPath/Structures/S_DamageInfo Structure") (`Damage Causer` :type "Actor Object Reference"))
  (returns (WasDamaged :type Boolean))
  (return false))

(fn `UserConstructionScript`
  (`parent.UserConstructionScript`))