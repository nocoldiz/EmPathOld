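; BP_SummonedDoor is a summoned portal door that sends the player to the RoomOverEdge level.
; On BeginPlay it destroys every other summoned door, so only the newest one remains.
; When the player pawn overlaps its Box, it messages the pawn to open RoomOverEdge, adding the MageGuid entrance when coming from another level.
; Returning to the previous door is still a TODO, and random door material assignment is disconnected.
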(event `self.ReceiveBeginPlay`
  (bind _outactors (`GameplayStatics.GetAllActorsOfClass` "BP_SummonedDoor_C"))
  (for _array_element _outactors
    (if (not (== _array_element self))
      (`self.K2_DestroyActor` _array_element)))
  (`parent.ReceiveBeginPlay`))

(event `self.Box.OnComponentBeginOverlap`
  (params (OverlappedComponent :type "PrimitiveComponent Object Reference") (OtherActor :type "Actor Object Reference") (OtherComp :type "PrimitiveComponent Object Reference") (OtherBodyIndex :type Integer) (bFromSweep :type Boolean) (SweepResult :type "HitResult Structure (by ref)"))
  (bind _returnvalue (`GameplayStatics.GetPlayerPawn` 0))
  (if (== OtherActor (`GameplayStatics.GetPlayerPawn` 0))
    (bind _returnvalue_2 (`GameplayStatics.GetCurrentLevelName` true))
    (if (`KismetStringLibrary.EqualEqual_StrStr` _returnvalue_2 "RoomOverEdge")
      (message `/Game/EmPath/Interfaces/BI_GameActions.OpenLevel` _returnvalue "RoomOverEdge" "" false false)
      (else
        (message `/Game/EmPath/Interfaces/BI_GameActions.OpenLevel` _returnvalue "RoomOverEdge" "MageGuid" false false) ; TODO: go back to previous door
      ))))

(fn `UserConstructionScript`
  (`parent.UserConstructionScript`))