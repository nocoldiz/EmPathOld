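; BP_Info is an interactable actor that displays an informational notice when used.
; The Use event passes its front, bold and body message text to Notice.
; Its construction script runs the parent setup and default constructions, then applies mesh, inspection and inventory settings.
; A Debug flag makes the Actor mesh component visible during construction.
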(event `/Game/HorrorEngine/Blueprints/Core/Use.Use`
  (params (HorrorEvent :type Boolean))
  ;[1 1 1] Take Settings
  (`/Game/HorrorEngine/Blueprints/Core/HorrorEngineFunctions.Notice` (`self.Front Message`) (`self.Bold Message`) (`self.Message`)))

(fn `UserConstructionScript`
  (`parent.UserConstructionScript`)
  (`/Game/HorrorEngine/Blueprints/Core/HorrorEngineMacros.HM_DefaultConstructions` _)
  (`/Game/HorrorEngine/Blueprints/Core/HorrorEngineFunctions.SetMesh` (`self.Actor`) (`self.MeshSettings`))
  (`self.SetInspection` (`self.InspectionSettings`))
  (`self.SetInventory` (`self.InventorySettings`))
  (if (`self.Debug`)
    (`SceneComponent.SetVisibility` (`self.Actor`) true false)))