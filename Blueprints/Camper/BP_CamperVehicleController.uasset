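; Camper vehicle Blueprint that drives the engine sound and exposes the camper's driving mode.
; Each tick, after the parent Tick, it scales the absolute forward speed from the vehicle movement component into the engine sound's RPM parameter, so pitch follows speed rather than simulated engine RPM.
; GetCamperMode returns the driving mode message read from player pawn 0, not from itself.
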(event `self.ReceiveTick`
  (params (DeltaSeconds :type "Float (single-precision)"))
  ;[1 1 1] Engine Sound
  (`parent.ReceiveTick` DeltaSeconds)
  (`AudioParameterControllerInterface.SetFloatParameter` (`self.EngineSound`) "RPM" (/ (`KismetMathLibrary.Abs` (`ChaosVehicleMovementComponent.GetForwardSpeed` (`self.VehicleMovementComponent`))) 7.0)))

(fn `GetCamperMode`
  (returns (CamperMode :type "/Game/EmPath/Enum/E_DrivingMode Enum"))
  (bind _drivingmode (message `/Game/EmPath/Interfaces/BI_GameActions.GetDrivingMode` (`GameplayStatics.GetPlayerPawn` 0)))
  (return _drivingmode))

(fn `UserConstructionScript`
  (`parent.UserConstructionScript`))