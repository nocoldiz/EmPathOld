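; Camper gravity button that switches gravity on every drivable actor and changes the player's driving mode.
; Overrides Use, calling the parent first, then finds all actors implementing BI_Drivable.
; For each, it sends SetGravity according to OnOff and sets one of two driving modes on player pawn 0.
; The pawn message sits inside the loop, so it repeats per drivable and never fires without one.
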(fn `Use`
  (params (HorrorEvent :type Boolean))
  (bind _returnvalue (`GameplayStatics.GetPlayerPawn` 0))
  (`parent.Use` HorrorEvent)
  (bind _outactors (`GameplayStatics.GetAllActorsWithInterface` "/Game/EmPath/Interfaces/BI_Drivable.BI_Drivable_C"))
  (for _array_element _outactors
    (if (`self.On / Off`)
      (message `/Game/EmPath/Interfaces/BI_Drivable.SetGravity` _array_element true)
      (message `/Game/EmPath/Interfaces/BI_GameActions.SetDrivingMode` _returnvalue "NewEnumerator6")
      (else
        (message `/Game/EmPath/Interfaces/BI_Drivable.SetGravity` _array_element false)
        (message `/Game/EmPath/Interfaces/BI_GameActions.SetDrivingMode` _returnvalue "NewEnumerator3")))))

(fn `UserConstructionScript`
  (`parent.UserConstructionScript`))