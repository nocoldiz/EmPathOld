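; BP_SteeringWheelAnimated is the camper's steering wheel actor, which visually turns in response to steering input.
; SteeringEvent receives an amount, scales it by a fixed factor and adds it as local roll to the Scene component, so rotation accumulates with each call.
; An RInterpTo-based return toward neutral rotation exists but is disconnected, so the wheel does not recenter by itself and Tick does nothing.
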(event `self.ReceiveTick`
  (params (DeltaSeconds :type "Float (single-precision)")))

(event `/Game/EmPath/Interfaces/BI_Drivable.SteeringEvent`
  (params (Amount :type "Float (double-precision)") (Flying :type Boolean))
  (`SceneComponent.K2_AddLocalRotation` (`self.Scene`) (`KismetMathLibrary.MakeRotator` (* Amount 4.0)) false false))

(fn `UserConstructionScript`)