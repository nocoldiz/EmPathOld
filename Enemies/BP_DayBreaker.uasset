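; BP_DayBreaker is an enemy Blueprint that exposes health through its BPCDamageSystem component.
; Its construction script runs the parent's, then sets the component's current Health to a fixed value, leaving MaxHealth untouched.
; GetCurrentHealth and GetMaxHealth read from that component, while Heal is a stub that returns zero.
; The event graph holds only disabled placeholder events, so it adds no behavior of its own.
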(fn `GetCurrentHealth`
  (returns (Health :type "Float (double-precision)"))
  (return (`/Game/EmPath/Blueprints/DamageSystem/BPC_DamageSystem.Health` (`self.BPC_DamageSystem`))))

(fn `GetMaxHealth`
  (returns (MaxHealth :type "Float (double-precision)"))
  (return (`/Game/EmPath/Blueprints/DamageSystem/BPC_DamageSystem.MaxHealth` (`self.BPC_DamageSystem`))))

(fn `Heal`
  (params (Amount :type "Float (double-precision)"))
  (returns (NewHealth :type "Float (double-precision)"))
  (return 0.0))

(fn `UserConstructionScript`
  (`parent.UserConstructionScript`)
  (set `/Game/EmPath/Blueprints/DamageSystem/BPC_DamageSystem.Health` 1000.0 (`self.BPC_DamageSystem`)))