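; Animal enemy Blueprint from the legacy melee enemy system, defining its attack set on top of a parent class.
; Attack events pass montage and damage info to BPCAttacks for ground smash, short, long and spinning melee, plus an ArcaneDart spell read from DT_Spells.
; It also sets fixed attack and defend ranges, caches mesh rotation at construction, and provides a helper predicting an actor's location from horizontal velocity.
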(event `self.ReceiveBeginPlay`
  (`parent.ReceiveBeginPlay`))

(event `CastSpell`
  (params (AttackTarget :type "Actor Object Reference"))
  ;[1 1 1] Attacks
  (bind _returnvalue (`|GetDataTableRow` "/Game/EmPath/DataTables/DT_Spells.DT_Spells" "ArcaneDart")
    (:`then`
      (`KismetSystemLibrary.PrintString` "Hello")
      (`/Game/EmPath/Enemies/LegacySystem/Attacks/BPC_Attacks.CastSpell` (`self.BPC_Attacks`) (make `/Game/EmPath/Structures/S_AttackInfo` AttackTarget "/Game/EmPath/Animations/Magic/Montage_Hadouken.Montage_Hadouken" (make `/Game/EmPath/Structures/S_DamageInfo` 0.0 "NewEnumerator1" "NewEnumerator0" false true)) 300.0 _returnvalue))))

(event `GroundSmashAttack`
  (params (AttackTarget :type "Actor Object Reference"))
  ;[1 1 1] Attacks
  (`/Game/EmPath/Enemies/LegacySystem/Attacks/BPC_Attacks.GroundSmash` (`self.BPC_Attacks`) (make `/Game/EmPath/Structures/S_AttackInfo` AttackTarget "/Game/EmPath/Animations/Melee/Montage_Melee_GroundSmash.Montage_Melee_GroundSmash" (make `/Game/EmPath/Structures/S_DamageInfo` 25.0 "NewEnumerator3")) 300.0))

(event `ShortRangeAttack`
  (params (AttackTarget :type "Actor Object Reference"))
  ;[1 1 1] Attacks
  (`/Game/EmPath/Enemies/LegacySystem/Attacks/BPC_Attacks.PrimaryMeleeAttack` (`self.BPC_Attacks`) (make `/Game/EmPath/Structures/S_AttackInfo` AttackTarget "/Game/EmPath/Animations/Melee/Montage_Sword_Slash.Montage_Sword_Slash" (make `/Game/EmPath/Structures/S_DamageInfo` 10.0 "NewEnumerator1" "NewEnumerator0" false true true)) 20.0 200.0))

(event `LongRangeAttack`
  (params (AttackTarget :type "Actor Object Reference"))
  ;[1 1 1] Attacks
  (`/Game/EmPath/Enemies/LegacySystem/Attacks/BPC_Attacks.LongRangeMeleeAttack` (`self.BPC_Attacks`) (make `/Game/EmPath/Structures/S_AttackInfo` AttackTarget "/Game/EmPath/Animations/Axe/Montage_Axe_Combo_1.Montage_Axe_Combo_1" (make `/Game/EmPath/Structures/S_DamageInfo` 10.0 "NewEnumerator1" "NewEnumerator0" false true true))))

(event `SpinningAttack`
  (params (AttackTarget :type "Actor Object Reference"))
  ;[1 1 1] Attacks
  (`/Game/EmPath/Enemies/LegacySystem/Attacks/BPC_Attacks.SpinningMeleeAttack` (`self.BPC_Attacks`) (make `/Game/EmPath/Structures/S_AttackInfo` AttackTarget "/Game/EmPath/Animations/Melee/Montage_Sword_SpinningAttack.Montage_Sword_SpinningAttack" (make `/Game/EmPath/Structures/S_DamageInfo` 10.0 "NewEnumerator1" "NewEnumerator0" false true))))

(fn `CalculateFutureActorLocation`
  (params (Actor :type "Actor Object Reference") (Time :type "Float (double-precision)" :default 1.0))
  (returns (Location :type "Vector Structure"))
  (return (+ (`self.K2_GetActorLocation` Actor) (* (* (`self.GetVelocity` Actor) (1.0 1.0 0.0)) Time))))

(fn `GetIdealRange`
  (returns (AttackRadius :type "Float (double-precision)") (DefendRadius :type "Float (double-precision)"))
  (return 200.0 400.0))

(fn `UserConstructionScript`
  (`parent.UserConstructionScript`)
  (set `self.MeshRotationBeforeSpin` (`SceneComponent.RelativeRotation` (`self.Mesh`))))