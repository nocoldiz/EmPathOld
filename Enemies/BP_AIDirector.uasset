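; AI director actor that keeps BP_FleshGoblin enemies spawning around the player on a looping timer.
; Each tick of the timer adds every living BPI_Damagable actor to SpawnedEnemies, which is never reset between passes.
; While that count is within MaxSpawnedEnemies, an inclusive loop over the shortfall spawns goblins at random navigable points near the player and prints their names.
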(event Custom|SpawnEnemies
  (bind _spawnedenemies (Variables|Default|GetSpawnedEnemies))
  (bind _maxspawnedenemies (Variables|Default|GetMaxSpawnedEnemies))
  (bind _returnvalue (- _maxspawnedenemies _spawnedenemies))
  (bind _outactors (Actor|GetAllActorswithInterface "/Game/EmPath/Interfaces/BPI_Damagable.BPI_Damagable_C"))
  (for _array_element _outactors
    (bind _health (Class|BPIDamagable|GetCurrentHealth(Message) _array_element))
    (if (> _health 0.0)
      (Math|Integer|IncrementInt (Variables|Default|GetSpawnedEnemies))))
  (if (>= _returnvalue 0)
    (for _index (range 0 _returnvalue)
      (bind _randomlocation (Class|NavigationSystemV1|GetRandomLocationinNavigableRadius (Transformation|GetActorLocation (Game|Player|GetPlayerPawn 0)) 2e+03 0 0))
      (bind _returnvalue_2 (Game|SpawnActorfromClass "/Game/EmPath/Enemies/BP_FleshGoblin.BP_FleshGoblin_C" (Math|Conversions|ToTransform(Vector) _randomlocation) "Undefined" "MultiplyWithRoot" 0 2 0 0 0 1e+03 0))
      (Development|PrintString (Utilities|GetDisplayName _returnvalue_2)))))

(event EventBeginPlay
  (Utilities|Time|SetTimerbyEvent (delegate Custom|SpawnEnemies) 1e+01 true))

(event Collision|EventActorBeginOverlap
  (params (OtherActor :type Actor%20Object%20Reference)))

(event EventTick
  (params (DeltaSeconds :type Float%20%28single-precision%29)))

(event Input|KeyboardEvents|DebugKeyNumPadNine
  (params (Key :type Key%20Structure :default "None") (ActionValue :type Input%20Action%20Value%20Structure)))

(fn ConstructionScript)