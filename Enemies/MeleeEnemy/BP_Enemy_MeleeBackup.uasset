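; Sword-wielding melee enemy, a child of a base enemy class, with ground smash, short-range slash, long-range jump and spinning attacks.
; Each attack event passes target, montage and damage info to the BPCAttacks component for execution.
; Montage notifies drive sword spawning onto the hand socket and its destruction, and montage completion fires equipped/unequipped callbacks.
; It also supplies ideal attack/defend ranges and a helper predicting an actor's future horizontal position from velocity.
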(event `self.ReceiveBeginPlay`
  (`parent.ReceiveBeginPlay`))

(event `GroundSmashAttack`
  (params (AttackTarget :type "Actor Object Reference"))
  ;[1 1 1] Attacks
  (`/Game/EmPath/Enemies/Attacks/BPC_Attacks.GroundSmash` (`self.BPC_Attacks`) (make `/Game/EmPath/Structures/S_AttackInfo` AttackTarget "/Game/EmPath/Animations/Melee/Montage_Melee_GroundSmash.Montage_Melee_GroundSmash" (make `/Game/EmPath/Structures/S_DamageInfo` 25.0 "NewEnumerator3")) 300.0))

(event `ShortRangeAttack`
  (params (AttackTarget :type "Actor Object Reference"))
  ;[1 1 1] Attacks
  (`/Game/EmPath/Enemies/Attacks/BPC_Attacks.PrimaryMeleeAttack` (`self.BPC_Attacks`) (make `/Game/EmPath/Structures/S_AttackInfo` AttackTarget "/Game/EmPath/Animations/Melee/Montage_Sword_Slash.Montage_Sword_Slash" (make `/Game/EmPath/Structures/S_DamageInfo` 10.0 "NewEnumerator1" "NewEnumerator0" false true true)) 20.0 200.0))

(event `LongRangeAttack`
  (params (AttackTarget :type "Actor Object Reference"))
  ;[1 1 1] Attacks
  (`/Game/EmPath/Enemies/Attacks/BPC_Attacks.LongRangeMeleeAttack` (`self.BPC_Attacks`) (make `/Game/EmPath/Structures/S_AttackInfo` AttackTarget "/Game/EmPath/Animations/Melee/Montage_Sword_Jump_Attack.Montage_Sword_Jump_Attack" (make `/Game/EmPath/Structures/S_DamageInfo` 10.0 "NewEnumerator1" "NewEnumerator0" false true true))))

(event `SpinningAttack`
  (params (AttackTarget :type "Actor Object Reference"))
  ;[1 1 1] Attacks
  (`/Game/EmPath/Enemies/Attacks/BPC_Attacks.SpinningMeleeAttack` (`self.BPC_Attacks`) (make `/Game/EmPath/Structures/S_AttackInfo` AttackTarget "/Game/EmPath/Animations/Melee/Montage_Sword_SpinningAttack.Montage_Sword_SpinningAttack" (make `/Game/EmPath/Structures/S_DamageInfo` 10.0 "NewEnumerator1" "NewEnumerator0" false true))))

(event `self.EquipWeapon`
  ;[1 1 1] Equip/Unequip weapon
  (bind _notifyname (`|PlayMontage` (`self.Mesh`) "/Game/EmPath/Animations/Melee/Montage_Unsheath_Sword.Montage_Unsheath_Sword")
    (:`OnCompleted`
      (`self.OnWeaponEquipped`))
    (:`OnNotifyBegin`
      (switch `name` _notifyname
        (:`HoldSword`
          (bind _returnvalue (`|SpawnActorFromClass` "/Game/EmPath/Enemies/Weapons/BP_Weapon_Sword.BP_Weapon_Sword_C" (`self.GetTransform`) "Undefined" "MultiplyWithRoot" null null))
          (bind _output_get (set `self.WeaponActor` _returnvalue))
          (`self.K2_AttachToComponent` _output_get (`self.Mesh`) "hand_r_sword_socket" "SnapToTarget" "SnapToTarget" "SnapToTarget" true)
          (set `self.IsWieldingWeapon` true))))))

(event `self.UnequipWeapon`
  ;[1 1 1] Equip/Unequip weapon
  (bind _notifyname (`|PlayMontage` (`self.Mesh`) "/Game/EmPath/Animations/Melee/Montage_Sheath_Sword.Montage_Sheath_Sword")
    (:`OnCompleted`
      (`self.OnWeaponUnequipped`))
    (:`OnNotifyBegin`
      (switch `name` _notifyname
        (:`DropSword`
          (`self.K2_DestroyActor` (`self.WeaponActor`))
          (set `self.IsWieldingWeapon` false))))))

(fn `CalculateFutureActorLocation`
  (params (Actor :type "Actor Object Reference") (Time :type "Float (double-precision)" :default 1.0))
  (returns (Location :type "Vector Structure"))
  (return (+ (`self.K2_GetActorLocation` Actor) (* (* (`self.GetVelocity` Actor) (1.0 1.0 0.0)) Time))))

(fn `GetIdealRange`
  (returns (AttackRadius :type "Float (double-precision)") (DefendRadius :type "Float (double-precision)"))
  (return 200.0 400.0))

(fn `UserConstructionScript`
  (`parent.UserConstructionScript`)
  (set `self.MeshRotationBeforeSpin` (`SceneComponent.RelativeRotation` (`self.Mesh`))))